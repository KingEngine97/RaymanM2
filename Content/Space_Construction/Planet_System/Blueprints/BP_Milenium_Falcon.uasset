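; Player-controlled Millennium Falcon ship with physics-based flight, steered by pitch, yaw and roll torques.
; Throttle input eases Thrust toward a target along the ship's forward vector; holding Supersonic speeds up the easing and pushes the target far beyond MaxThrust.
; Tick overwrites the body's linear velocity with forward velocity plus a simulated gravity fall that grows below GravityThreshold and eases out above it.
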(event EventBeginPlay
  ;[1 1 1] Set_Thrust
  (Variables|Default|SetThrust (/ (Variables|Default|GetMaxThrust) 2.0)))

(event Collision|EventActorBeginOverlap
  (params (OtherActor :type Actor%20Object%20Reference)))

(event EventTick
  (params (DeltaSeconds :type Float%20%28single-precision%29))
  ;[1 1 1] Velocity and Rotation
  (Utilities|FlowControl|Sequence
    (:then_0
      (if (< (Math|Vector|VectorLength (Variables|Default|GetForwardVelocity)) (Variables|Default|GetGravityThreshold))
        (Variables|Default|SetUpwardsVelocity (* (Math|Vector|UnrotateVector (Math|Vector|GetUpVector (Variables|Default|GetShip)) (Transformation|GetWorldRotation (Variables|Default|GetShip))) (Math|Float|Lerp 0.0 -9.8e+02 (- 1.0 (/ (Math|Vector|VectorLength (Variables|Default|GetForwardVelocity)) (Variables|Default|GetGravityThreshold))))))
        (else
          (Variables|Default|SetUpwardsVelocity (Math|Interpolation|VInterpTo (Variables|Default|GetUpwardsVelocity) "0, 0, 0" (Utilities|Time|GetWorldDeltaSeconds) 2e+01)))))
    (:then_1
      (Physics|SetPhysicsLinearVelocity (Variables|Default|GetShip) (+ (Variables|Default|GetForwardVelocity) (Variables|Default|GetUpwardsVelocity)) false "None"))))

(event Input|ActionEvents|InputActionSupersonic?
  (params (Key :type Key%20Structure))
  ;[1 1 1] Super_Speed
  (:Pressed
    (bind _output_get (Variables|Default|SetSuperspeed true)))
  (:Released
    (Variables|Default|SetSuperspeed false)))

(event Input|AxisEvents|InputAxisThrust
  (params (AxisValue :type Float%20%28single-precision%29))
  ;[1 1 1] Thrust_Speed
  (Utilities|FlowControl|Sequence
    (:then_0
      (if (stale Input|ActionEvents|InputActionSupersonic? _output_get)
        ;[1 1 1] Super_Speed
        (if (not (Math|Float|NearlyEqual(Float) AxisValue 0.0 0.1))
          (Variables|Default|SetThrust (Math|Interpolation|FInterpTo (Variables|Default|GetThrust) (Math|Float|Lerp 0.0 (Variables|Default|GetMaxThrust) (/ (+ AxisValue 1.0) 0.1)) (Utilities|Time|GetWorldDeltaSeconds) 2.0)))
        (elif (not (Math|Float|NearlyEqual(Float) AxisValue 0.0 0.1))
          (Variables|Default|SetThrust (Math|Interpolation|FInterpTo (Variables|Default|GetThrust) (Math|Float|Lerp 0.0 (Variables|Default|GetMaxThrust) (/ (+ AxisValue 1.0) 2.0)) (Utilities|Time|GetWorldDeltaSeconds) 0.5)))))
    (:then_1
      (Variables|Default|SetForwardVelocity (* (Math|Vector|GetForwardVector (Variables|Default|GetShip)) (Variables|Default|GetThrust))))))

(event Input|AxisEvents|InputAxisMoveUp
  (params (AxisValue :type Float%20%28single-precision%29))
  ;[1 1 1] Move_Up
  (Class|PrimitiveComponent|AddTorqueinDegrees (Variables|Default|GetShip) (* (Math|Vector|GetRightVector (Variables|Default|GetShip)) (* AxisValue (Variables|Default|GetForwardTorquePower))) "None" true))

(event Input|AxisEvents|InputAxisMoveRight
  (params (AxisValue :type Float%20%28single-precision%29))
  ;[1 1 1] Move_Left_Right
  (Class|PrimitiveComponent|AddTorqueinDegrees (Variables|Default|GetShip) (* (Math|Vector|GetUpVector (Variables|Default|GetShip)) (* AxisValue (Variables|Default|GetSideTorquePower))) "None" true))

(event Input|AxisEvents|InputAxisRoll
  (params (AxisValue :type Float%20%28single-precision%29))
  ;[1 1 1] Roll
  (Class|PrimitiveComponent|AddTorqueinDegrees (Variables|Default|GetShip) (* (Math|Vector|GetForwardVector (Variables|Default|GetShip)) (* (Math|Float|Clamp(Float) AxisValue -1.0) (Variables|Default|GetRotationTorque))) "None" true))

(fn ConstructionScript)