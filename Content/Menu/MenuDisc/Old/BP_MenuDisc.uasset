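; BP_MenuDisc is a 3D holographic menu disc actor that hosts a Menu3DWidget and links to other menu actors.
; BeginPlay hides flagged elements, disables collision and binds the widget's transition event.
; Transitions move collision to the indexed linked menu and blend the camera view to it.
; Sequence playback, portal material lerps and button effects are disconnected, most click handlers are empty, and Quit requires a flag that only disconnected code sets.
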(event Custom|TransitionTo
  (params (Transition%20Target :type BP%20Menu%20Disc%20Object%20Reference))
  ;[1 1 1] TransitionTo (Target)
  (Collision|SetActorEnableCollision false)
  (Collision|SetActorEnableCollision Transition%20Target true)
  (Game|Player|SetViewTargetwithBlend (Game|GetPlayerController 0) Transition%20Target 1.0 "VTBlend_Cubic" 0.0 false))

(event Custom|HideWidget
  ;[1 1 1] Hide Widget
  (if (Variables|Default|GetHIDE_Widget)
    (Development|SetHiddeninGame (Variables|Default|GetWidget) true false)))

(event Custom|Hide_Elements
  (CallFunction|HideHomeDisc)
  (CallFunction|HideCharDisc)
  (CallFunction|HideWidget))

(event Custom|On%20Transition%20Between%20Menus
  (params (MenuIndex :type Integer))
  ;[1 1 1] Begin Play
  (if (Utilities|Array|IsValidIndex (Variables|Default|GetLinkedMenus) MenuIndex)
    (CallFunction|Transitionto (Utilities|Array|Get(acopy) (Variables|Default|GetLinkedMenus) MenuIndex))))

(event Custom|On%20Clicked%20%28ButtonNEWGAME%29
  ;[0.224 0.3031 1] Click New Game
)

(event Custom|HideHomeDisc
  ;[1 1 1] HideHomeDisc
  (if (Variables|Default|GetHIDE_HomeDisc)
    (for _array_element (Utilities|Array|MakeArray (Variables|Default|GetM2_HomeDisc_Inner_Laser) (Variables|Default|GetM2_HomeDisc_Display_Border_W) (Variables|Default|GetM2_HomeDisc_Border_L) (Variables|Default|GetM2_HomeDisc_Outer_Laser_Seam) (Variables|Default|GetM2_HomeDisc_Object_1) (Variables|Default|GetFlashlight3) (Variables|Default|GetVFX2%20) (Variables|Default|GetVFX) (Variables|Default|GetVFX1%20) (Variables|Default|GetBackgroundDisc))
      (Development|SetHiddeninGame _array_element true false))))

(event Custom|Click%20Quit%20Game
  ;[0.224 0.3031 1] Quit Game
  (if (Variables|HOME|GetisPlaying_SEQ_HOME)
    (Variables|HOME|SetisPlaying_SEQ_HOME false)
    (Game|QuitGame 0 "Quit" false)))

(event Custom|Click%20Settings
  ;[0.224 0.3031 1] Click Settings
)

(event Custom|Click%20Load%20Game
  ;[0.224 0.3031 1] Load Game
)

(event Custom|HideCharDisc
  ;[1 1 1] Hide Char Disc
  (if (Variables|Default|GetHIDE_CharDisc)
    (Development|SetHiddeninGame (Variables|Default|GetM2_CharDisc) true false)))

(event EventTick
  (params (DeltaSeconds :type Float%20%28single-precision%29))
  ;[1 1 1] EventTick
  (if (Variables|HOME|GetisPlaying_SEQ_HOME)
    (Variables|Components|SetHologram_ALL (Utilities|Array|MakeArray 0 0 0 0 0))
    (else
      (Components|Activation|Deactivate (Variables|Default|GetDefaultSceneRoot)))))

(event EventBeginPlay
  ;[1 1 1] Begin Play
  (CallFunction|HideElements)
  (bind _asmenu_3dwidget (Utilities|Casting|CastToMenu3DWidget (UserInterface|GetUserWidgetObject (Variables|Default|GetWidget))))
  (EventDispatchers|AssignTransitiontoLinkedMenu _asmenu_3dwidget (delegate Custom|On%20Transition%20Between%20Menus))
  (Collision|SetActorEnableCollision false))

(fn ConstructionScript)

(fn PlaySequence
  (params (Level%20Sequence :type Level%20Sequence%20Object%20Reference) (Settings%20Loop :type Movie%20Scene%20Sequence%20Loop%20Count%20Structure))
  (bind _outactor (Sequencer|Player|CreateLevelSequencePlayer Level%20Sequence (Utilities|Struct|MakeMovieSceneSequencePlaybackSettings false Settings%20Loop 1.0 0.0 false false false false false false false false)))
  (Sequencer|Player|Play (Variables|/Script/LevelSequence.LevelSequenceActor|GetSequencePlayer _outactor) :!class /Script/MovieScene.MovieSceneSequencePlayer)
  (return (Media|MediaPlayer|GetDuration (Variables|/Script/LevelSequence.LevelSequenceActor|GetSequencePlayer _outactor)) (Variables|/Script/LevelSequence.LevelSequenceActor|GetSequencePlayer _outactor)))