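; 3D menu disc actor that serves as one screen in a set of linked in-world menus.
; On BeginPlay it optionally hides home or character disc meshes and binds to its Menu3DWidget, whose transition event moves collision and blends the camera to an indexed linked menu.
; ActivatePortal drives circle, laser and hologram material parameters from one timeline.
; Quit is conditional; other click handlers are empty, and the Level Sequence lookup is disconnected.
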(event Custom|ActivatePortal
  (bind _mesh_bigcircle_c (Variables|Default|GetMesh_BigCircle_C))
  (bind _hologram_all (Variables|Components|GetHologram_ALL))
  (bind _mesh_laserbeam_1a (Variables|Default|GetMesh_Laserbeam_1A))
  (bind _mesh_laserbeam_1b (Variables|Default|GetMesh_Laserbeam_1B))
  (bind _mesh_bigcircle_a (Variables|Default|GetMesh_BigCircle_A))
  (bind _mesh_smallcircle (Variables|Default|GetMesh_SmallCircle))
  ;[1 1 1] Activate Portal
  ;;[0.4914 1 0.5337] Small Circle
  (bind _alpha (Timeline|Emissive+Hue Play)
    (:Update
      (Utilities|LerpScalarMaterialParameterValues _mesh_smallcircle "Hue" 0.0 0.4 _alpha)
      (Utilities|LerpScalarMaterialParameterValues _mesh_smallcircle "Emissive" 1.0 5.0 _alpha)
      ;;[0.4914 1 0.5337] Laserbeam 1A
      (Utilities|LerpScalarMaterialParameterValues _mesh_laserbeam_1a "Hue" 0.04 0.54 _alpha)
      (Utilities|LerpScalarMaterialParameterValues _mesh_laserbeam_1a "Hue" 0.1 0.6 _alpha)
      (Utilities|LerpVectorMaterialParameterValues _mesh_laserbeam_1a "ScrollDirection" "0.000000,-1.000000,0.000000" "0.000000,-5.000000,0.000000" _alpha)
      ;;[0.4914 1 0.5337] Laserbeam 1B
      (Utilities|LerpScalarMaterialParameterValues _mesh_laserbeam_1b "Hue" 0.04 0.54 _alpha)
      (Utilities|LerpScalarMaterialParameterValues _mesh_laserbeam_1b "Hue" 0.1 0.6 _alpha)
      (Utilities|LerpVectorMaterialParameterValues _mesh_laserbeam_1b "ScrollDirection" "0.000000,-1.000000,0.000000" "0.000000,-5.000000,0.000000" _alpha)
      ;;[0.4914 1 0.5337] Big Circle A
      (Utilities|LerpVectorMaterialParameterValues _mesh_bigcircle_a "Color1" "0.420000,0.040000,0.000000" "0.000000,0.250000,1.000000" _alpha)
      (Utilities|LerpScalarMaterialParameterValues _mesh_bigcircle_a "Radius" 0.3 0.5 _alpha)
      (Utilities|LerpScalarMaterialParameterValues _mesh_bigcircle_a "X Tile Speed" -0.02 -0.3 _alpha)
      (Utilities|LerpScalarMaterialParameterValues _mesh_bigcircle_a "X Tile Speed (2)" 0.02 0.3 _alpha)
      ;;[0.4914 1 0.5337] Big Circle B
      (Utilities|LerpScalarMaterialParameterValues (Variables|Default|GetMesh_BigCircle_B) "Radius" 0.5 0.0 _alpha)
      ;;[0.4914 1 0.5337] Big Circle C
      (Utilities|LerpScalarMaterialParameterValues _mesh_bigcircle_c "Radius" 1.0 0.0 _alpha)
      (Utilities|LerpScalarMaterialParameterValues _mesh_bigcircle_c "Hue" -0.4 0.2 _alpha)
      ;;[0.4914 1 0.5337] Hologram
      (Utilities|LerpARRAYScalarMaterialParameter _hologram_all "Erode" 1.0 -0.1 _alpha)
      (Utilities|LerpARRAYScalarMaterialParameter _hologram_all "Emissive" 5.0 0.01 _alpha)
      ;;[0.4914 1 0.5337] Buttons
      (Rendering|Material|SetMaterial (Utilities|Array|MakeArray 0 0 0 0 0) 0 "/Game/Materials/Gradient/MAT_Invisible.MAT_Invisible")
      ;;[0.4914 1 0.5337] Flashlight
      (Rendering|Material|SetMaterial (Utilities|Array|MakeArray (Variables|Default|GetFlashlight1) (Variables|Default|GetFlashlight2) (Variables|Default|GetFlashlight3)) 0 "/Game/Menu/MenuDisc/Mat/FLIP_Flashlight_Inst.FLIP_Flashlight_Inst"))))

(event Custom|TransitionTo
  (params (Transition%20Target :type BP%20Menu%20Disc%20Object%20Reference))
  ;[1 1 1] TransitionTo (Target)
  (Collision|SetActorEnableCollision false)
  (Collision|SetActorEnableCollision Transition%20Target true)
  (Game|Player|SetViewTargetwithBlend (Game|GetPlayerController 0) Transition%20Target 1.0 "VTBlend_Cubic" 0.0 false))

(event Custom|On%20Transition%20Between%20Menus
  (params (MenuIndex :type Integer))
  ;[1 1 1] Begin Play
  (if (Utilities|Array|IsValidIndex (Variables|Default|GetLinkedMenus) MenuIndex)
    (CallFunction|Transitionto (Utilities|Array|Get(acopy) (Variables|Default|GetLinkedMenus) MenuIndex))))

(event Custom|On%20Clicked%20%28ButtonNEWGAME%29
  ;[0.224 0.3031 1] Click New Game
)

(event Custom|HideHomeDisc
  ;[1 1 1] HideHomeDisc
  (if (Variables|Default|GetHIDE_HomeDisc)
    (for _array_element (Utilities|Array|MakeArray (Variables|Default|GetMenuDisc_Box_E) (Variables|Default|GetMenuDisc_Eye_NW_2) (Variables|Default|GetMenuDisc_Eye_SW) (Variables|Default|GetMenuDisc_Eye_SW_2) (Variables|Default|GetMenuDisc_Inner_Border) (Variables|Default|GetMesh_SmallCircle) (Variables|Default|GetMesh_Laserbeam_1B) (Variables|Default|GetMenuDisc_Eye_east) (Variables|Default|GetMenuDisc_Circuit_NW_13) (Variables|Default|GetMenuDisc_Circuit_NW_14) (Variables|Default|GetMenuDisc_Display_Border_W) (Variables|Default|GetMenuDisc_Display_Border_W_2) (Variables|Default|GetMenuDisc_Display_S) (Variables|Default|GetMenuDisc_Display_S_Border) (Variables|Default|GetMenuDisc_Display_W) (Variables|Default|GetMenuDisc_Object_9) (Variables|Default|GetMenuDisc_Object_10) (Variables|Default|GetMenuDisc_Object_11) (Variables|Default|GetMenuDisc_Object_12) (Variables|Default|GetMenuDisc_Object_14) (Variables|Default|GetMenuDisc_Object_15) (Variables|Default|GetMenuDisc_Object_16) (Variables|Default|GetMenuDisc_Object_8) (Variables|Default|GetMenuDisc_Object_1) (Variables|Default|GetMenuDisc_Object_2) (Variables|Default|GetMenuDisc_Object_3) (Variables|Default|GetMenuDisc_Object_4) (Variables|Default|GetMesh_Laserbeam_1A) (Variables|Default|GetMenuDisc_Object_5) (Variables|Default|GetMenuDisc_Object_6) (Variables|Default|GetMenuDisc_Object_7) (Variables|Default|GetMenuDisc_Circuit_NW_12) (Variables|Default|GetMenuDisc_Button_S_2) (Variables|Default|GetMenuDisc_Button_Small_E) (Variables|Default|GetMenuDisc_Button_Small_E_2) (Variables|Default|GetMenuDisc_Button_Small_E_3) (Variables|Default|GetMenuDisc_Button_Small_E_4) (Variables|Default|GetMenuDisc_Button_Small_E_5) (Variables|Default|GetMenuDisc_Button_Small_E_6) (Variables|Default|GetMenuDisc_Button_S) (Variables|Default|GetMenuDisc_Border_L) (Variables|Default|GetHOME_Screw%201) (Variables|Default|GetMenuDisc_Box_Laser) (Variables|Default|GetMenuDisc_Box_N) (Variables|Default|GetMenuDisc_Box_NW) (Variables|Default|GetMenuDisc_Button_E) (Variables|Default|GetMenuDisc_Button_E_2) (Variables|Default|GetMenuDisc_Button_Small_S) (Variables|Default|GetMenuDisc_Circuit_NW_4) (Variables|Default|GetMenuDisc_Circuit_NW_5) (Variables|Default|GetMenuDisc_Circuit_NW_6) (Variables|Default|GetMenuDisc_Circuit_NW_7) (Variables|Default|GetMenuDisc_Circuit_NW_8) (Variables|Default|GetMenuDisc_Circuit_NW_9) (Variables|Default|GetMenuDisc_Circuit_NW_10) (Variables|Default|GetMenuDisc_Circuit_NW_3) (Variables|Default|GetMenuDisc_Button_Small_S_2) (Variables|Default|GetMenuDisc_Button_W) (Variables|Default|GetMenuDisc_Button_W_2) (Variables|Default|GetMenuDisc_Button_WSW) (Variables|Default|GetMenuDisc_Circuit_NW_11) (Variables|Default|GetMenuDisc_Button_WSW_2) (Variables|Default|GetMenuDisc_Circuit_NW) (Variables|Default|GetMenuDisc_Circuit_NW_2) (Variables|Default|GetButtonsFix_Slot3) (Variables|Default|GetMenuDiscButtonsFix_Object_1) (Variables|Default|GetMenuDiscButtonsFix_Object_2) (Variables|Default|GetButtonsFix_Slot2_2) (Variables|Default|GetMenuDiscButtonsFix_Object_3) (Variables|Default|GetMenuDiscButtonsFix_Object_4) (Variables|Default|GetMenuDiscButtonsFix_Object_5) (Variables|Default|GetMenuDisc_Small_Buttons_N_5) (Variables|Default|GetMenuDisc_Small_Buttons_N_6) (Variables|Default|GetButtonsFix_Slot1) (Variables|Default|GetMenuDiscButtonsFix_Object_6) (Variables|Default|GetButtonsFix_Slot4) (Variables|Default|GetButtonsFix_Slot5) (Variables|Default|GetButtonsFix_Slot6) (Variables|Default|GetButtonsFix_Slot7) (Variables|Default|GetFlashlight1) (Variables|Default|GetFlashlight2) (Variables|Default|GetFlashlight3) (Variables|Default|GetMesh_BigCircle_C) (Variables|Default|GetMenuDisc_Object_20) (Variables|Default|GetMenuDiscButtonsFix_Object_7) (Variables|Default|GetHologram1) (Variables|Default|GetHologram7) (Variables|Default|GetHologram6) (Variables|Default|GetMenuDisc_Small_Buttons_N_4) (Variables|Default|GetHologram4) (Variables|Default|GetHologram3) (Variables|Default|GetMesh_BigCircle_A) (Variables|Default|GetMesh_BigCircle_B) (Variables|Default|GetMenuDisc_Object_17) (Variables|Default|GetMenuDisc_Object_26) (Variables|Default|GetMenuDisc_Object_27) (Variables|Default|GetMenuDisc_Pipe_Circle_Big) (Variables|Default|GetMenuDisc_Pipe_Circle_Small) (Variables|Default|GetMenuDisc_Pipe_S) (Variables|Default|GetMenuDisc_Pipe_W) (Variables|Default|GetMenuDisc_Pipes_E) (Variables|Default|GetMenuDisc_Object_25) (Variables|Default|GetMenuDisc_Object_18) (Variables|Default|GetMenuDisc_Object_19) (Variables|Default|GetBackgroundDisc) (Variables|Default|GetMenuDisc_Object_21) (Variables|Default|GetMenuDisc_Object_22) (Variables|Default|GetMenuDisc_Object_23) (Variables|Default|GetMenuDisc_Object_24) (Variables|Default|GetMenuDisc_Pipes_N) (Variables|Default|GetMenuDisc_Pipes_NE_6) (Variables|Default|GetMenuDisc_Pipes_NE_7) (Variables|Default|GetMenuDisc_Pipes_NE_8) (Variables|Default|GetMenuDisc_Pipes_NE_9) (Variables|Default|GetMenuDisc_Screen_at_NW) (Variables|Default|GetMenuDisc_Small_Buttons_N) (Variables|Default|GetMenuDisc_Small_Buttons_N_2) (Variables|Default|GetMenuDisc_Pipes_NE_5) (Variables|Default|GetMenuDisc_Pipes_N_2) (Variables|Default|GetMenuDisc_Pipes_N_3) (Variables|Default|GetMenuDisc_Pipes_N_4) (Variables|Default|GetMenuDisc_Pipes_NE) (Variables|Default|GetMenuDisc_Small_Buttons_N_3) (Variables|Default|GetMenuDisc_Pipes_NE_2) (Variables|Default|GetMenuDisc_Pipes_NE_3) (Variables|Default|GetMenuDisc_Pipes_NE_4) 0)
      (Development|SetHiddeninGame _array_element true false))))

(event Custom|Click%20Quit%20Game
  ;[0.224 0.3031 1] Quit Game
  (if (Variables|HOME|GetisPlaying_SEQ_HOME)
    (Variables|HOME|SetisPlaying_SEQ_HOME false)
    (Game|QuitGame 0 "Quit" false)))

(event Custom|Click%20Settings
  ;[0.224 0.3031 1] Click Settings
)

(event Custom|Click%20Load%20Game
  ;[0.224 0.3031 1] Load Game
)

(event Custom|HideCharDisc
  ;[1 1 1] Hide Char Disc
  (if (Variables|Default|GetHIDE_CharDisc)
    (Development|SetHiddeninGame (Variables|Default|GetM2_CharDisc) true false)))

(event EventTick
  (params (DeltaSeconds :type Float%20%28single-precision%29))
  ;[1 1 1] EventTick
  (if (Variables|HOME|GetisPlaying_SEQ_HOME)
    (Variables|Components|SetHologram_ALL (Utilities|Array|MakeArray (Variables|Default|GetHologram1) (Variables|Default|GetHologram3) (Variables|Default|GetHologram4) (Variables|Default|GetHologram6) (Variables|Default|GetHologram7)))
    (else
      (Components|Activation|Deactivate (Variables|Default|GetDefaultSceneRoot)))))

(event EventBeginPlay
  ;[1 1 1] Begin Play
  (CallFunction|HideHomeDisc)
  (CallFunction|HideCharDisc)
  (bind _asmenu_3dwidget (Utilities|Casting|CastToMenu3DWidget (UserInterface|GetUserWidgetObject (Variables|Default|GetWidget))))
  (EventDispatchers|AssignTransitiontoLinkedMenu _asmenu_3dwidget (delegate Custom|On%20Transition%20Between%20Menus))
  (Collision|SetActorEnableCollision false))

(fn ConstructionScript)

(fn PlaySequence
  (params (Level%20Sequence :type Level%20Sequence%20Object%20Reference) (Settings%20Loop :type Movie%20Scene%20Sequence%20Loop%20Count%20Structure))
  (bind _outactor (Sequencer|Player|CreateLevelSequencePlayer Level%20Sequence (Utilities|Struct|MakeMovieSceneSequencePlaybackSettings false Settings%20Loop 1.0 0.0 false false false false false false false false)))
  (Sequencer|Player|Play (Variables|/Script/LevelSequence.LevelSequenceActor|GetSequencePlayer _outactor) :!class /Script/MovieScene.MovieSceneSequencePlayer)
  (return (Media|MediaPlayer|GetDuration (Variables|/Script/LevelSequence.LevelSequenceActor|GetSequencePlayer _outactor)) (Variables|/Script/LevelSequence.LevelSequenceActor|GetSequencePlayer _outactor)))