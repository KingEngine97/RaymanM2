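; Character disc for the menu, handling cursor hover and click selection of Rayman through level sequences.
; Hovering the picture or icon prints the component name and plays the hover sequence once, guarded by hovered and selected flags.
; Leaving the icon stops it and plays SEQOnline.
; The icon's click branch would play the select sequence and set the classic skin, but a constant false condition keeps it from running.
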(event OnBeginCursorOver(CharacterDisc_Ico_ray)
  (params (TouchedComponent :type Primitive%20Component%20Object%20Reference))
  (Development|PrintString (Utilities|GetDisplayName TouchedComponent))
  ;[1 1 1] Rayman
  ;;[1 1 1] OnHovered >> IF IsHovered: false >> Play Rayman Intro Sequence  >> Set IsHovered: true
  (if (not (stale OnClicked(CharacterDisc_Ico_ray) _output_get))
    (if (not (stale _output_get))
      (bind _outactor (Sequencer|Player|CreateLevelSequencePlayer (Variables|Default|GetSEQ%20CHAR%20Rayman%20on%20Hover)))
      (Sequencer|Player|Play (Variables|/Script/LevelSequence.LevelSequenceActor|GetSequencePlayer _outactor) :!class /Script/MovieScene.MovieSceneSequencePlayer)
      (bind _output_get (Variables|Default|SetIs%20Hovered%20Rayman true)))))

(event OnEndCursorOver(CharacterDisc_Ico_ray)
  (params (TouchedComponent :type Primitive%20Component%20Object%20Reference))
  ;[1 1 1] Rayman
  ;;[1 1 1] OnUnhovered >> IF IsHovered: true >> Stop Rayman Intro Sequence >> Set IsHovered: false
  (if true
    (Sequencer|Player|Stop (Variables|/Script/LevelSequence.LevelSequenceActor|GetSequencePlayer (stale OnBeginCursorOver(CharacterDisc_Ico_ray) _outactor)) :!class /Script/MovieScene.MovieSceneSequencePlayer)
    (bind _outactor (Sequencer|Player|CreateLevelSequencePlayer (Variables|Default|GetSEQ_Online)))
    (Sequencer|Player|Play (Variables|/Script/LevelSequence.LevelSequenceActor|GetSequencePlayer _outactor) :!class /Script/MovieScene.MovieSceneSequencePlayer)
    (Variables|Default|SetIs%20Hovered%20Rayman false)))

(event OnClicked(CharacterDisc_Ico_ray)
  (params (TouchedComponent :type Primitive%20Component%20Object%20Reference) (ButtonPressed :type Key%20Structure :default "None"))
  ;[1 1 1] Rayman
  ;;[1 1 1] OnClicked >> IF IsHovered: true && IF NOT IsSelected: true >> Stop Rayman Intro Sequence >> Play Rayman Select Sequence
  (if (and false (not (stale _output_get)))
    (Sequencer|Player|Stop (Variables|/Script/LevelSequence.LevelSequenceActor|GetSequencePlayer (stale OnBeginCursorOver(CharacterDisc_Ico_ray) _outactor)) :!class /Script/MovieScene.MovieSceneSequencePlayer)
    (bind _outactor (Sequencer|Player|CreateLevelSequencePlayer (Variables|Default|GetSEQ%20CHAR%20Rayman%20on%20Click)))
    (Sequencer|Player|Play (Variables|/Script/LevelSequence.LevelSequenceActor|GetSequencePlayer _outactor) :!class /Script/MovieScene.MovieSceneSequencePlayer)
    (bind _output_get (Variables|Default|SetIs%20Selected%20Rayman true))
    (Variables|Default|SetSKIN%20RAY%20Classic? true)))

(event OnBeginCursorOver(CharacterDisc_window_picture)
  (params (TouchedComponent :type Primitive%20Component%20Object%20Reference))
  (Development|PrintString (Utilities|GetDisplayName (stale OnBeginCursorOver(CharacterDisc_Ico_ray) TouchedComponent)))
  ;[1 1 1] Rayman
  ;;[1 1 1] OnHovered >> IF IsHovered: false >> Play Rayman Intro Sequence  >> Set IsHovered: true
  (if (not (stale OnClicked(CharacterDisc_Ico_ray) _output_get))
    (if (not (stale _output_get))
      (bind _outactor (Sequencer|Player|CreateLevelSequencePlayer (Variables|Default|GetSEQ%20CHAR%20Rayman%20on%20Hover)))
      (Sequencer|Player|Play (Variables|/Script/LevelSequence.LevelSequenceActor|GetSequencePlayer _outactor) :!class /Script/MovieScene.MovieSceneSequencePlayer)
      (bind _output_get (Variables|Default|SetIs%20Hovered%20Rayman true)))))

(fn ConstructionScript)