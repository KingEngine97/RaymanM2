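; Rayman's thrown hand, an actor parented to Rayman_BP that flies out as a punch projectile and returns to its socket.
; ThrowHand hides the hand bones, then a timeline moves it straight toward the target, or along a spline for aimed strafing attacks.
; Overlaps deal damage, spawn impact effects, push plums and reverse the timeline early.
; The return tracks the moving socket, then reattaches; a cable shows for one power-up.
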(event OnComponentBeginOverlap(Sphere)
  (params (OverlappedComponent :type Primitive%20Component%20Object%20Reference) (OtherActor :type Actor%20Object%20Reference) (OtherComp :type Primitive%20Component%20Object%20Reference) (OtherBodyIndex :type Integer) (bFromSweep :type Boolean) (SweepResult :type Hit%20Result%20Structure%20%28by%20ref%29))
  (if (Variables|Default|GetBusy)
    (if (Math|Boolean|ANDBoolean (!= OtherActor (Game|GetPlayerCharacter 0)) (!= OtherActor self) (!= OtherActor "RaymanHand_BP"))
      (Variables|/Script/Engine.PrimitiveComponent|SetbGenerateOverlapEvents (Variables|Default|GetSphere) false)
      (Utilities|IsValid OtherActor
        (:Is%20Valid
          (Class|RaymanInterface|CauseDamage(Message) OtherActor (Variables|Default|GetDamage)))
        (:Is%20Not%20Valid
          _))
      (Utilities|Casting|CastToCharacter OtherActor
        (:then
          (Niagara|SpawnSystematLocation "/Game/Z_Add-Ons/AdvancedMagicFX13/Particles/Niagara/NS_ky_impact.NS_ky_impact" (Transformation|GetActorLocation) "0, 0, 0" "0.500000,0.500000,0.500000"))
        (:CastFailed
          (Utilities|Casting|CastToRaymanHand_BP OtherActor
            (:CastFailed
              (Utilities|Casting|CastToSwimmableWater OtherActor
                (:CastFailed
                  (bind _asplum_bp (Utilities|Casting|CastToPlum_BP OtherActor)
                    (:then
                      (Physics|AddImpulse (Variables|/Game/Z_Add-Ons/LumenEngine/Plum_BP.Plum_BP_C|GetBox _asplum_bp) (* (* (Math|Rotator|GetRotationXVector (Math|Rotator|FindLookatRotation (Transformation|GetActorLocation) (Transformation|GetActorLocation _asplum_bp))) 1e+01) (* (Variables|Default|GetDamage) 10)) "None" true))
                    (:CastFailed
                      _))
                  (Niagara|SpawnSystematLocation "/Game/Z_Add-Ons/A_Surface_Footstep/Niagara_FX/ParticleSystems/PSN_General1_Surface.PSN_General1_Surface" (Transformation|GetActorLocation))))))))
      (CallFunction|ForceReturnHand))))

(event Custom|ThrowHand
  (params (AttackStartLocation :type Vector) (AttackTargetLocation :type Vector) (Damage :type Integer) (Spline :type Spline%20Component%20Object%20Reference))
  (bind _rayman_player (Variables|Default|GetRayman_Player))
  (bind _rayman_player_2 (Variables|Default|GetRayman_Player))
  (bind _rayman_player_3 (Variables|Default|GetRayman_Player))
  (bind _rayman_player_4 (Variables|Default|GetRayman_Player))
  (bind _target (Variables|/Game/Z_Add-Ons/LumenEngine/Characters/Rayman/Rayman_BP.Rayman_BP_C|GetTarget _rayman_player_4))
  (bind _returnvalue (Transformation|GetActorLocation _target))
  (Variables|Default|SetDamage Damage)
  (Variables|Default|SetSpline Spline)
  (Rendering|SetVisibility (Variables|Default|GetStaticMesh) true false)
  (if (> (Variables|Default|GetDamage) 15)
    (Audio|SpawnSoundAttached "/Game/Z_Add-Ons/LumenEngine/Audio/SFX/_extracted/4758126.4758126" (Variables|Default|GetStaticMesh) "None" "0, 0, 0" "0, 0, 0" "KeepRelativeOffset" false 1.0 1.0 0.0 "/Game/Z_Add-Ons/LumenEngine/Audio/Normal_Attenuation.Normal_Attenuation" 0)
    (else
      (Audio|SpawnSoundAttached "/Game/Z_Add-Ons/LumenEngine/Audio/SFX/_extracted/35650270.35650270" (Variables|Default|GetStaticMesh) "None" "0, 0, 0" "0, 0, 0" "KeepRelativeOffset" false 1.0 1.0 0.0 "/Game/Z_Add-Ons/LumenEngine/Audio/Normal_Attenuation.Normal_Attenuation" 0)))
  (Variables|/Script/Engine.PrimitiveComponent|SetbGenerateOverlapEvents (Variables|Default|GetSphere) true)
  (Variables|Default|SetBusy true)
  (Variables|Default|SetAttack%20Start%20Location AttackStartLocation)
  (Utilities|IsValid _target
    (:Is%20Valid
      (bind _output_get (Variables|Default|SetAiming (Variables|/Game/Z_Add-Ons/LumenEngine/Characters/Rayman/Rayman_BP.Rayman_BP_C|GetAiming _rayman_player_4)))
      (if _output_get
        (if (== (Variables|/Game/Z_Add-Ons/LumenEngine/Characters/Rayman/Rayman_BP.Rayman_BP_C|GetMoveRight/Left _rayman_player_4) 0.0)
          (Variables|Default|SetAiming false :!label _label)
          (Variables|Default|SetAttack%20Target%20Location _returnvalue)
          (bind _output_get_2 (Variables|Default|SetHandRotation (Math|Rotator|FindLookatRotation (Variables|Default|GetAttack%20Start%20Location) (Variables|Default|GetAttack%20Target%20Location))))
          (Variables|Default|SetAttack%20Target%20Location (+ (Variables|Default|GetAttack%20Target%20Location) (* (Math|Vector|GetForwardVector _output_get_2) (- 9e+02 (Math|Vector|Distance(Vector) (Variables|Default|GetAttack%20Start%20Location) (Variables|Default|GetAttack%20Target%20Location))))))
          (else
            (Default|StrafeSplineAttack _rayman_player_4)
            (Variables|Default|SetAttack%20Target%20Location _returnvalue)
            (Variables|Default|SetHandRotation (Math|Rotator|FindLookatRotation (Variables|Default|GetAttack%20Start%20Location) (Variables|Default|GetAttack%20Target%20Location)))
            (Variables|Default|SetAttack%20Target%20Location (Transformation|GetActorLocation _target))))
        (else
          (goto _label))))
    (:Is%20Not%20Valid
      (Variables|Default|SetAiming false)
      (Variables|Default|SetAttack%20Target%20Location AttackTargetLocation)
      (Variables|Default|SetHandRotation (Math|Rotator|FindLookatRotation (Variables|Default|GetAttack%20Start%20Location) (Variables|Default|GetAttack%20Target%20Location)))))
  (Transformation|DetachFromComponent (Variables|Default|GetSphere) "KeepWorld" "KeepWorld" "KeepWorld" true)
  (Components|SkinnedMesh|HideBonebyName (Variables|/Script/Engine.Character|GetMesh (Variables|Default|GetRayman_Player)) (Utilities|Select :Index (Variables|Default|GetHandIndex) :Option%200 "Channel-11" :Option%201 "Channel-10") "PBO_None")
  (Components|SkinnedMesh|HideBonebyName (Variables|/Script/Engine.Character|GetMesh (Variables|Default|GetRayman_Player)) (Utilities|Select :Index (Variables|Default|GetHandIndex) :Option%200 "Channel-5" :Option%201 "Channel-4") "PBO_None")
  (Components|SkinnedMesh|HideBonebyName (Variables|/Script/Engine.Character|GetMesh (Variables|Default|GetRayman_Player)) (Utilities|Select :Index (Variables|Default|GetHandIndex) :Option%200 "Channel-20" :Option%201 "Channel-19") "PBO_None")
  (Rendering|SetVisibility (Variables|Default|GetCable) (Utilities|Enum|Equal(Enum) (Variables|/Game/Z_Add-Ons/LumenEngine/Characters/Rayman/Rayman_BP.Rayman_BP_C|GetCurrentPowerUp _rayman_player_4) "NewEnumerator0") false)
  (bind _newtrack_0 (Timeline|Timeline_0 PlayFromStart)
    (:Update
      (if (>= (Components|Timeline|GetPlaybackPosition (Variables|Default|GetTimeline_0)) 0.5)
        (Variables|Default|SetAttack%20Start%20Location (Transformation|GetWorldLocation (Utilities|Select :Index (Variables|Default|GetHandIndex) :Option%200 (Variables|/Game/Z_Add-Ons/LumenEngine/Characters/Rayman/Rayman_BP.Rayman_BP_C|GetRightHandSocket _rayman_player_3) :Option%201 (Variables|/Game/Z_Add-Ons/LumenEngine/Characters/Rayman/Rayman_BP.Rayman_BP_C|GetLeftHandSocket _rayman_player_3))))
        (Transformation|SetActorLocation (.Location (Math|Transform|BreakTransform (Math|Transform|Lerp(Transform) (Math|Transform|MakeTransform (Variables|Default|GetAttack%20Start%20Location) (Math|Rotator|MakeRotator (+ (.Roll (Math|Rotator|BreakRotator (Variables|Default|GetHandRotation))) 9e+01) (+ (.Pitch (Math|Rotator|BreakRotator (Variables|Default|GetHandRotation))) 1.8e+02) (+ (.Yaw (Math|Rotator|BreakRotator (Variables|Default|GetHandRotation))) 9e+01))) (Math|Transform|MakeTransform (Variables|Default|GetAttack%20Target%20Location) (Math|Rotator|MakeRotator (+ (.Roll (Math|Rotator|BreakRotator (Variables|Default|GetHandRotation))) 9e+01) (+ (.Pitch (Math|Rotator|BreakRotator (Variables|Default|GetHandRotation))) 1.8e+02) (+ (.Yaw (Math|Rotator|BreakRotator (Variables|Default|GetHandRotation))) 9e+01))) _newtrack_0))) true false)
        (Transformation|SetActorRotation (.Rotation (Math|Transform|BreakTransform (Math|Transform|Lerp(Transform) (Math|Transform|MakeTransform (Variables|Default|GetAttack%20Start%20Location) (Math|Rotator|MakeRotator (+ (.Roll (Math|Rotator|BreakRotator (Variables|Default|GetHandRotation))) 9e+01) (+ (.Pitch (Math|Rotator|BreakRotator (Variables|Default|GetHandRotation))) 1.8e+02) (+ (.Yaw (Math|Rotator|BreakRotator (Variables|Default|GetHandRotation))) 9e+01))) (Math|Transform|MakeTransform (Variables|Default|GetAttack%20Target%20Location) (Math|Rotator|MakeRotator (+ (.Roll (Math|Rotator|BreakRotator (Variables|Default|GetHandRotation))) 9e+01) (+ (.Pitch (Math|Rotator|BreakRotator (Variables|Default|GetHandRotation))) 1.8e+02) (+ (.Yaw (Math|Rotator|BreakRotator (Variables|Default|GetHandRotation))) 9e+01))) _newtrack_0))))
        (elif (Variables|Default|GetAiming)
          (Transformation|SetActorLocation (Spline|GetLocationatDistanceAlongSpline (Variables|Default|GetSpline) (Math|Float|Lerp 0.0 (Spline|GetDistanceAlongSplineatSplinePoint (Variables|Default|GetSpline) 2) _newtrack_0) "World") true false)
          (Transformation|SetActorRotation (Math|Conversions|RotationFromXVector (Spline|GetDirectionatDistanceAlongSpline (Variables|Default|GetSpline) (Math|Float|Lerp 0.0 (Spline|GetDistanceAlongSplineatSplinePoint (Variables|Default|GetSpline) 2) _newtrack_0) "World")))
          (else
            (Transformation|SetActorLocation (.Location (Math|Transform|BreakTransform (Math|Transform|Lerp(Transform) (Math|Transform|MakeTransform (Variables|Default|GetAttack%20Start%20Location) (Math|Rotator|MakeRotator (+ (.Roll (Math|Rotator|BreakRotator (Variables|Default|GetHandRotation))) 9e+01) (+ (.Pitch (Math|Rotator|BreakRotator (Variables|Default|GetHandRotation))) 1.8e+02) (+ (.Yaw (Math|Rotator|BreakRotator (Variables|Default|GetHandRotation))) 9e+01))) (Math|Transform|MakeTransform (Variables|Default|GetAttack%20Target%20Location) (Math|Rotator|MakeRotator (+ (.Roll (Math|Rotator|BreakRotator (Variables|Default|GetHandRotation))) 9e+01) (+ (.Pitch (Math|Rotator|BreakRotator (Variables|Default|GetHandRotation))) 1.8e+02) (+ (.Yaw (Math|Rotator|BreakRotator (Variables|Default|GetHandRotation))) 9e+01))) _newtrack_0))) true false)
            (Transformation|SetActorRotation (.Rotation (Math|Transform|BreakTransform (Math|Transform|Lerp(Transform) (Math|Transform|MakeTransform (Variables|Default|GetAttack%20Start%20Location) (Math|Rotator|MakeRotator (+ (.Roll (Math|Rotator|BreakRotator (Variables|Default|GetHandRotation))) 9e+01) (+ (.Pitch (Math|Rotator|BreakRotator (Variables|Default|GetHandRotation))) 1.8e+02) (+ (.Yaw (Math|Rotator|BreakRotator (Variables|Default|GetHandRotation))) 9e+01))) (Math|Transform|MakeTransform (Variables|Default|GetAttack%20Target%20Location) (Math|Rotator|MakeRotator (+ (.Roll (Math|Rotator|BreakRotator (Variables|Default|GetHandRotation))) 9e+01) (+ (.Pitch (Math|Rotator|BreakRotator (Variables|Default|GetHandRotation))) 1.8e+02) (+ (.Yaw (Math|Rotator|BreakRotator (Variables|Default|GetHandRotation))) 9e+01))) _newtrack_0))))
            (Utilities|FlowControl|Gate true :!label _label_2
              (:Exit
                (Variables|Default|SetAttack%20Start%20Location (Transformation|GetWorldLocation (Utilities|Select :Index (Variables|Default|GetHandIndex) :Option%200 (Variables|/Game/Z_Add-Ons/LumenEngine/Characters/Rayman/Rayman_BP.Rayman_BP_C|GetRightHandSocket _rayman_player_2) :Option%201 (Variables|/Game/Z_Add-Ons/LumenEngine/Characters/Rayman/Rayman_BP.Rayman_BP_C|GetLeftHandSocket _rayman_player_2))))))))))
    (:Finished
      (Transformation|AttachComponentToComponent (Utilities|Select :Index (Variables|Default|GetHandIndex) :Option%200 (Variables|/Game/Z_Add-Ons/LumenEngine/Characters/Rayman/Rayman_BP.Rayman_BP_C|GetRightHandSocket _rayman_player) :Option%201 (Variables|/Game/Z_Add-Ons/LumenEngine/Characters/Rayman/Rayman_BP.Rayman_BP_C|GetLeftHandSocket _rayman_player)) "None" "SnapToTarget" "SnapToTarget" "KeepWorld" true)
      (Variables|Default|SetBusy false)
      (Rendering|SetVisibility (Variables|Default|GetStaticMesh) false false)
      (Variables|/Script/Engine.PrimitiveComponent|SetbGenerateOverlapEvents (Variables|Default|GetSphere) false)
      (Components|SkinnedMesh|UnHideBonebyName (Variables|/Script/Engine.Character|GetMesh _rayman_player) (Utilities|Select :Index (Variables|Default|GetHandIndex) :Option%200 "Channel-11" :Option%201 "Channel-10"))
      (Components|SkinnedMesh|UnHideBonebyName (Variables|/Script/Engine.Character|GetMesh _rayman_player) (Utilities|Select :Index (Variables|Default|GetHandIndex) :Option%200 "Channel-5" :Option%201 "Channel-4"))
      (Components|SkinnedMesh|UnHideBonebyName (Variables|/Script/Engine.Character|GetMesh _rayman_player) (Utilities|Select :Index (Variables|Default|GetHandIndex) :Option%200 "Channel-20" :Option%201 "Channel-19"))
      (Rendering|SetVisibility (Variables|Default|GetCable) false false)
      (goto _label_2 Close))))

(event Custom|ForceReturnHand
  (bind _rayman_player (Variables|Default|GetRayman_Player))
  (bind _rayman_player_2 (Variables|Default|GetRayman_Player))
  (bind _handrotation (Variables|Default|GetHandRotation))
  (bind _rayman_player_3 (Variables|Default|GetRayman_Player))
  (bind _spline (Variables|Default|GetSpline))
  (bind (_roll _pitch _yaw) (Math|Rotator|BreakRotator _handrotation))
  (bind _returnvalue (+ _pitch 1.8e+02))
  (bind _returnvalue_2 (+ _roll 9e+01))
  (bind _returnvalue_3 (+ _yaw 9e+01))
  (bind _returnvalue_4 (Math|Rotator|MakeRotator _returnvalue_2 _returnvalue _returnvalue_3))
  (Utilities|FlowControl|Delay 0.065)
  (if (Variables|Default|GetAiming)
    (Variables|Default|SetAttack%20Start%20Location (Transformation|GetActorLocation (Game|GetPlayerCharacter 0)))
    (Variables|Default|SetAiming false))
  (Utilities|FlowControl|Sequence
    (:then_0
      (bind _newtrack_0 (Timeline|Timeline_0 Reverse)
        (:Update
          (if (>= (Components|Timeline|GetPlaybackPosition (Variables|Default|GetTimeline_0)) 0.5)
            (Variables|Default|SetAttack%20Start%20Location (Transformation|GetWorldLocation (Utilities|Select :Index (Variables|Default|GetHandIndex) :Option%200 (Variables|/Game/Z_Add-Ons/LumenEngine/Characters/Rayman/Rayman_BP.Rayman_BP_C|GetRightHandSocket _rayman_player_3) :Option%201 (Variables|/Game/Z_Add-Ons/LumenEngine/Characters/Rayman/Rayman_BP.Rayman_BP_C|GetLeftHandSocket _rayman_player_3))))
            (Transformation|SetActorLocation (.Location (Math|Transform|BreakTransform (Math|Transform|Lerp(Transform) (Math|Transform|MakeTransform (Variables|Default|GetAttack%20Start%20Location) _returnvalue_4) (Math|Transform|MakeTransform (Variables|Default|GetAttack%20Target%20Location) _returnvalue_4) _newtrack_0))) true false)
            (Transformation|SetActorRotation (.Rotation (Math|Transform|BreakTransform (Math|Transform|Lerp(Transform) (Math|Transform|MakeTransform (Variables|Default|GetAttack%20Start%20Location) _returnvalue_4) (Math|Transform|MakeTransform (Variables|Default|GetAttack%20Target%20Location) _returnvalue_4) _newtrack_0))))
            (elif (Variables|Default|GetAiming)
              (Transformation|SetActorLocation (Spline|GetLocationatDistanceAlongSpline _spline (Math|Float|Lerp 0.0 (Spline|GetDistanceAlongSplineatSplinePoint _spline 2) _newtrack_0) "World") true false)
              (Transformation|SetActorRotation (Math|Conversions|RotationFromXVector (Spline|GetDirectionatDistanceAlongSpline _spline (Math|Float|Lerp 0.0 (Spline|GetDistanceAlongSplineatSplinePoint _spline 2) _newtrack_0) "World")))
              (else
                (Transformation|SetActorLocation (.Location (Math|Transform|BreakTransform (Math|Transform|Lerp(Transform) (Math|Transform|MakeTransform (Variables|Default|GetAttack%20Start%20Location) _returnvalue_4) (Math|Transform|MakeTransform (Variables|Default|GetAttack%20Target%20Location) _returnvalue_4) _newtrack_0))) true false)
                (Transformation|SetActorRotation (.Rotation (Math|Transform|BreakTransform (Math|Transform|Lerp(Transform) (Math|Transform|MakeTransform (Variables|Default|GetAttack%20Start%20Location) _returnvalue_4) (Math|Transform|MakeTransform (Variables|Default|GetAttack%20Target%20Location) _returnvalue_4) _newtrack_0))))
                (Utilities|FlowControl|Gate true :!label _label
                  (:Exit
                    (Variables|Default|SetAttack%20Start%20Location (Transformation|GetWorldLocation (Utilities|Select :Index (Variables|Default|GetHandIndex) :Option%200 (Variables|/Game/Z_Add-Ons/LumenEngine/Characters/Rayman/Rayman_BP.Rayman_BP_C|GetRightHandSocket _rayman_player_2) :Option%201 (Variables|/Game/Z_Add-Ons/LumenEngine/Characters/Rayman/Rayman_BP.Rayman_BP_C|GetLeftHandSocket _rayman_player_2))))))))))
        (:Finished
          (Transformation|AttachComponentToComponent (Utilities|Select :Index (Variables|Default|GetHandIndex) :Option%200 (Variables|/Game/Z_Add-Ons/LumenEngine/Characters/Rayman/Rayman_BP.Rayman_BP_C|GetRightHandSocket _rayman_player) :Option%201 (Variables|/Game/Z_Add-Ons/LumenEngine/Characters/Rayman/Rayman_BP.Rayman_BP_C|GetLeftHandSocket _rayman_player)) "None" "SnapToTarget" "SnapToTarget" "KeepWorld" true)
          (Variables|Default|SetBusy false)
          (Rendering|SetVisibility (Variables|Default|GetStaticMesh) false false)
          (Variables|/Script/Engine.PrimitiveComponent|SetbGenerateOverlapEvents (Variables|Default|GetSphere) false)
          (Components|SkinnedMesh|UnHideBonebyName (Variables|/Script/Engine.Character|GetMesh _rayman_player) (Utilities|Select :Index (Variables|Default|GetHandIndex) :Option%200 "Channel-11" :Option%201 "Channel-10"))
          (Components|SkinnedMesh|UnHideBonebyName (Variables|/Script/Engine.Character|GetMesh _rayman_player) (Utilities|Select :Index (Variables|Default|GetHandIndex) :Option%200 "Channel-5" :Option%201 "Channel-4"))
          (Components|SkinnedMesh|UnHideBonebyName (Variables|/Script/Engine.Character|GetMesh _rayman_player) (Utilities|Select :Index (Variables|Default|GetHandIndex) :Option%200 "Channel-20" :Option%201 "Channel-19"))
          (Rendering|SetVisibility (Variables|Default|GetCable) false false)
          (goto _label Close))))
    (:then_1
      (goto _label Open))))

(event EventBeginPlay
  (bind _asrayman_bp (Utilities|Casting|CastToRayman_BP (Actor|GetParentActor)))
  (Variables|Default|SetRayman_Player _asrayman_bp))

(fn ConstructionScript
  (Class|CableComponent|SetAttachEndto (Variables|Default|GetCable) (Actor|GetParentActor) "None" "None"))