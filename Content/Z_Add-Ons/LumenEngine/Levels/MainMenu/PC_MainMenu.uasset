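; Player controller for the main menu level that routes menu navigation input to the main menu widget.
; Shortly after BeginPlay it finds the existing top-level W_MainMenu instance and caches it, rather than creating one itself.
; The up, down, left, right and select input actions each call the matching highlight or select function on that widget, which handles the menu logic.
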(event EventBeginPlay
  (Utilities|FlowControl|Delay 0.2)
  (bind _foundwidgets (Widget|GetAllWidgetsOfClass "/Game/Z_Add-Ons/LumenEngine/Levels/MainMenu/W_MainMenu.W_MainMenu_C" true))
  (Variables|Default|SetMainMenu_Widget (Utilities|Array|Get(acopy) _foundwidgets)))

(event Input|ActionEvents|InputActionMenu_Up
  (params (Key :type Key%20Structure))
  (:Pressed
    (Default|HighlightOptionUp (Variables|Default|GetMainMenu_Widget))))

(event Input|ActionEvents|InputActionMenu_Down
  (params (Key :type Key%20Structure))
  (:Pressed
    (Default|HighlightOptionDown (Variables|Default|GetMainMenu_Widget))))

(event Input|ActionEvents|InputActionMenu_Select
  (params (Key :type Key%20Structure))
  (:Pressed
    (Default|SelectOption (Variables|Default|GetMainMenu_Widget))))

(event Input|ActionEvents|InputActionMenu_Left
  (params (Key :type Key%20Structure))
  (:Pressed
    (Default|HighlightLeftOption (Variables|Default|GetMainMenu_Widget))))

(event Input|ActionEvents|InputActionMenu_Right
  (params (Key :type Key%20Structure))
  (:Pressed
    (Default|HighlightRightOption (Variables|Default|GetMainMenu_Widget))))

(fn ConstructionScript)