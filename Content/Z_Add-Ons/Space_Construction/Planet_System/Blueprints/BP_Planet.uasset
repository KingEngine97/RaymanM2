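; Planet actor that builds a configurable planet with atmosphere and rings for space scenes, set up entirely in the construction script.
; It creates dynamic materials for the three meshes, then pushes exposed color, atmosphere, cloud and ring settings into them.
; The atmosphere mesh scales from planet radius and height, and all three materials take their light vector from the referenced SunLight's rotation.
; Ring shape and shadow parameters are mirrored into the atmosphere material.
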(event EventBeginPlay)

(fn ConstructionScript
  (bind _sunlight (Variables|Default|GetSunLight))
  (bind _returnvalue (Transformation|GetActorRotation _sunlight))
  (bind _returnvalue_2 (Math|Rotator|GetRotationXVector _returnvalue))
  (bind _returnvalue_3 (* _returnvalue_2 -1.0))
  (bind _returnvalue_4 (Math|Conversions|ToLinearColor(Vector) _returnvalue_3))
  (Utilities|FlowControl|Sequence
    (:then_0
      ;[1 1 1] Create Dynamic Material Instances
      (bind _returnvalue_5 (Rendering|Material|CreateDynamicMaterialInstance (Variables|Default|GetAtmosphere) 0 (Variables|Materials|GetAtmosphere%20Material) "None" :!class /Script/Engine.PrimitiveComponent))
      (Variables|Default|SetDMI_Atmosphere _returnvalue_5)
      (bind _returnvalue_6 (Rendering|Material|CreateDynamicMaterialInstance (Variables|Default|GetPlanet) 0 (Variables|Materials|GetPlanet%20Material) "None" :!class /Script/Engine.PrimitiveComponent))
      (Variables|Default|SetDMI_Planet _returnvalue_6)
      (bind _returnvalue_7 (Rendering|Material|CreateDynamicMaterialInstance (Variables|Default|GetRings) 0 (Variables|Materials|GetRings%20Material) "None" :!class /Script/Engine.PrimitiveComponent))
      (Variables|Default|SetDMI_Rings _returnvalue_7))
    (:then_1
      ;[1 1 1] Loc/Scale
      (Rendering|Material|SetVectorParameterValue (Variables|Default|GetDMI_Atmosphere) "PlanetLocation" (Math|Conversions|ToLinearColor(Vector) (Transformation|GetWorldLocation (Variables|Default|Getroot))) :!class /Script/Engine.MaterialInstanceDynamic)
      (Rendering|Material|SetScalarParameterValue (Variables|Default|GetDMI_Atmosphere) "Radius" (* (Variables|Default|GetPlanetRadius) 2.0 (.y (Variables|/Script/Engine.SceneComponent|GetRelativeScale3D (Variables|Default|Getroot self)))) :!class /Script/Engine.MaterialInstanceDynamic)
      ;[1 1 1] Light Direction
      (Rendering|Material|SetVectorParameterValue (Variables|Default|GetDMI_Atmosphere) "Light Vector" (Math|Conversions|ToLinearColor(Vector) (* _returnvalue_2 -1.0)) :!class /Script/Engine.MaterialInstanceDynamic)
      (Rendering|Material|SetVectorParameterValue (Variables|Default|GetDMI_Planet) "Light Vector" _returnvalue_4 :!class /Script/Engine.MaterialInstanceDynamic)
      (Rendering|Material|SetVectorParameterValue (Variables|Default|GetDMI_Rings) "Light_Vector" _returnvalue_4 :!class /Script/Engine.MaterialInstanceDynamic))
    (:then_2
      ;[1 1 1] Atmosphere
      (Rendering|Material|SetScalarParameterValue (Variables|Default|GetDMI_Atmosphere) "AtmosphereHeight" (Variables|Atmosphere|GetAtmosphereHeight) :!class /Script/Engine.MaterialInstanceDynamic)
      (Transformation|SetRelativeScale3D (Variables|Default|GetAtmosphere) (Math|Conversions|ToVector(Float) (+ (* (Variables|Atmosphere|GetAtmosphereHeight) 0.016) (Variables|Default|GetPlanetRadius))))
      (Rendering|Material|SetScalarParameterValue (Variables|Default|GetDMI_Atmosphere) "Atmosphere Steps" (Math|Conversions|ToFloat(Integer) (Math|Float|Round (Variables|Atmosphere|GetAtmosphere%20Steps))) :!class /Script/Engine.MaterialInstanceDynamic)
      (Rendering|Material|SetVectorParameterValue (Variables|Default|GetDMI_Atmosphere) "Scattering_Color" (Variables|Atmosphere|GetScattering%20Color) :!class /Script/Engine.MaterialInstanceDynamic)
      (Rendering|Material|SetVectorParameterValue (Variables|Default|GetDMI_Planet) "Scattering_Color" (Variables|Atmosphere|GetScattering%20Color) :!class /Script/Engine.MaterialInstanceDynamic)
      (Rendering|Material|SetVectorParameterValue (Variables|Default|GetDMI_Atmosphere) "Atmosphere Night Color" (Variables|Atmosphere|GetNight%20Color) :!class /Script/Engine.MaterialInstanceDynamic)
      (Rendering|Material|SetVectorParameterValue (Variables|Default|GetDMI_Planet) "Night Color" (Variables|Atmosphere|GetNight%20Color) :!class /Script/Engine.MaterialInstanceDynamic)
      (Rendering|Material|SetVectorParameterValue (Variables|Default|GetDMI_Planet) "Sunset Color 1" (Variables|Atmosphere|GetSunset%20Color%201) :!class /Script/Engine.MaterialInstanceDynamic)
      (Rendering|Material|SetVectorParameterValue (Variables|Default|GetDMI_Planet) "Sunset Color 2" (Variables|Atmosphere|GetSunset%20Color%202) :!class /Script/Engine.MaterialInstanceDynamic))
    (:then_3
      ;[1 1 1] Global
      (Rendering|Material|SetScalarParameterValue (Variables|Default|GetDMI_Planet) "Global Clouds Ratio" (Variables|Default|GetGlobal%20Tile%20Ratio) :!class /Script/Engine.MaterialInstanceDynamic))
    (:then_4
      ;[1 1 1] Rings
      (Rendering|Material|SetScalarParameterValue (Variables|Default|GetDMI_Rings) "Inner Edge" (Variables|Rings|GetInner%20Edge) :!class /Script/Engine.MaterialInstanceDynamic)
      (Rendering|Material|SetScalarParameterValue (Variables|Default|GetDMI_Rings) "Outer Edge" (Variables|Rings|GetOuter%20Edge) :!class /Script/Engine.MaterialInstanceDynamic)
      (Rendering|Material|SetScalarParameterValue (Variables|Default|GetDMI_Rings) "Frequency_1" (Variables|Rings|GetFrequency%201) :!class /Script/Engine.MaterialInstanceDynamic)
      (Rendering|Material|SetScalarParameterValue (Variables|Default|GetDMI_Rings) "Frequency_2" (Variables|Rings|GetFrequency%202) :!class /Script/Engine.MaterialInstanceDynamic)
      (Rendering|Material|SetScalarParameterValue (Variables|Default|GetDMI_Rings) "Density" (Variables|Rings|GetDensity) :!class /Script/Engine.MaterialInstanceDynamic)
      (Rendering|Material|SetScalarParameterValue (Variables|Default|GetDMI_Rings) "Seed" (Variables|Rings|GetSeed) :!class /Script/Engine.MaterialInstanceDynamic)
      (Rendering|Material|SetScalarParameterValue (Variables|Default|GetDMI_Rings) "Rings Edge Hardness" (Variables|Rings|GetEdge%20Hardness) :!class /Script/Engine.MaterialInstanceDynamic)
      (Rendering|Material|SetScalarParameterValue (Variables|Default|GetDMI_Rings) "Shadow Strength" (Variables|Rings|GetShadow%20Strength) :!class /Script/Engine.MaterialInstanceDynamic)
      (Rendering|Material|SetScalarParameterValue (Variables|Default|GetDMI_Rings) "Shadow Hardness" (Variables|Rings|GetShadow%20Hardness) :!class /Script/Engine.MaterialInstanceDynamic)
      (Rendering|Material|SetScalarParameterValue (Variables|Default|GetDMI_Rings) "Scattering Size" (Variables|Rings|GetScattering%20Size) :!class /Script/Engine.MaterialInstanceDynamic)
      (Rendering|Material|SetScalarParameterValue (Variables|Default|GetDMI_Rings) "Scattering Power" (Variables|Rings|GetScattering%20Power) :!class /Script/Engine.MaterialInstanceDynamic)
      (Rendering|Material|SetVectorParameterValue (Variables|Default|GetDMI_Rings) "Color_1" (Variables|Rings|GetRings%20Color%201) :!class /Script/Engine.MaterialInstanceDynamic)
      (Rendering|Material|SetVectorParameterValue (Variables|Default|GetDMI_Rings) "Color_2" (Variables|Rings|GetRings%20Color%202) :!class /Script/Engine.MaterialInstanceDynamic)
      (Rendering|Material|SetVectorParameterValue (Variables|Default|GetDMI_Rings) "Color_3" (Variables|Rings|GetRings%20Color%203) :!class /Script/Engine.MaterialInstanceDynamic)
      (Rendering|Material|SetVectorParameterValue (Variables|Default|GetDMI_Rings) "Color_4" (Variables|Rings|GetRings%20Color%204) :!class /Script/Engine.MaterialInstanceDynamic)
      (Rendering|Material|SetVectorParameterValue (Variables|Default|GetDMI_Rings) "Scattering Color" (Variables|Rings|GetRings%20Scatering%20Color) :!class /Script/Engine.MaterialInstanceDynamic))
    (:then_5
      (Rendering|Material|SetScalarParameterValue (Variables|Default|GetDMI_Atmosphere) "Inner Edge" (Variables|Rings|GetInner%20Edge) :!class /Script/Engine.MaterialInstanceDynamic)
      (Rendering|Material|SetScalarParameterValue (Variables|Default|GetDMI_Atmosphere) "Outer Edge" (Variables|Rings|GetOuter%20Edge) :!class /Script/Engine.MaterialInstanceDynamic)
      (Rendering|Material|SetScalarParameterValue (Variables|Default|GetDMI_Atmosphere) "Frequency_1" (Variables|Rings|GetFrequency%201) :!class /Script/Engine.MaterialInstanceDynamic)
      (Rendering|Material|SetScalarParameterValue (Variables|Default|GetDMI_Atmosphere) "Frequency_2" (Variables|Rings|GetFrequency%202) :!class /Script/Engine.MaterialInstanceDynamic)
      (Rendering|Material|SetScalarParameterValue (Variables|Default|GetDMI_Atmosphere) "Density" (Variables|Rings|GetDensity) :!class /Script/Engine.MaterialInstanceDynamic)
      (Rendering|Material|SetScalarParameterValue (Variables|Default|GetDMI_Atmosphere) "Seed" (Variables|Rings|GetSeed) :!class /Script/Engine.MaterialInstanceDynamic)
      (Rendering|Material|SetScalarParameterValue (Variables|Default|GetDMI_Atmosphere) "Rings Edge Hardness" (Variables|Rings|GetEdge%20Hardness) :!class /Script/Engine.MaterialInstanceDynamic)
      (Rendering|Material|SetScalarParameterValue (Variables|Default|GetDMI_Atmosphere) "Shadow Strength" (Variables|Rings|GetShadow%20Strength) :!class /Script/Engine.MaterialInstanceDynamic)
      (Rendering|Material|SetScalarParameterValue (Variables|Default|GetDMI_Atmosphere) "Shadow Hardness" (Variables|Rings|GetShadow%20Hardness) :!class /Script/Engine.MaterialInstanceDynamic)
      (Rendering|Material|SetScalarParameterValue (Variables|Default|GetDMI_Atmosphere) "Scattering Size" (Variables|Rings|GetScattering%20Size) :!class /Script/Engine.MaterialInstanceDynamic)
      (Rendering|Material|SetScalarParameterValue (Variables|Default|GetDMI_Atmosphere) "Scattering Power" (Variables|Rings|GetScattering%20Power) :!class /Script/Engine.MaterialInstanceDynamic))))