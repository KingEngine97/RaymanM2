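; Space scene actor that builds a forming star with a surrounding disk and fog, or a collapsed mass with gravitational lensing.
; The construction script pushes exposed variables into dynamic materials on an inverted sphere (disk, lighting, cubemaps, background stars) and the star mesh (surface, flares, atmosphere).
; Collapse zero-scales the star and applies lensing; otherwise StarSize drives mesh scale, mass and Niagara sun rays.
; Runtime events are empty.
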(event EventBeginPlay)

(event Collision|EventActorBeginOverlap
  (params (OtherActor :type Actor%20Object%20Reference)))

(event EventTick
  (params (DeltaSeconds :type Float%20%28single-precision%29)))

(fn ConstructionScript
  (bind _invertedspherehq (Variables|Default|GetInvertedSphereHQ))
  (bind _star_mesh (Variables|Default|GetStar_Mesh))
  (bind _starsize (Variables|Matter&Mass|GetStarSize))
  (bind _invertedspherehq_2 (Variables|Default|GetInvertedSphereHQ))
  (bind _invertedspherehq_3 (Variables|Default|GetInvertedSphereHQ))
  (Utilities|FlowControl|Sequence
    (:then_0
      (bind _returnvalue (Rendering|Material|CreateDynamicMaterialInstance (Variables|Default|GetInvertedSphereHQ) 0 "/Game/Z_Add-Ons/Space_Construction/Planet_System/Materials/Star/MI_M_Star_Fuel.MI_M_Star_Fuel" "None" :!class /Script/Engine.PrimitiveComponent))
      (Utilities|FlowControl|Sequence
        (:then_0
          ;[1 1 1] Material_Setup
          (Rendering|Material|SetScalarParameterValueonMaterials _invertedspherehq_2 "Disk Density" (Variables|GasDisk|GetDisk%20Density))
          (Rendering|Material|SetScalarParameterValueonMaterials _invertedspherehq_2 "Disk Density Bias" (Variables|GasDisk|GetDisk%20Density%20Bias))
          (Rendering|Material|SetScalarParameterValueonMaterials _invertedspherehq_2 "Disk Density Inner Radius" (Variables|GasDisk|GetDisk%20Density%20Inner%20Radius))
          (Rendering|Material|SetScalarParameterValueonMaterials _invertedspherehq_2 "Disk Density Outer Radius" (Variables|GasDisk|GetDisk%20Density%20Outer%20Radius))
          (Rendering|Material|SetScalarParameterValueonMaterials _invertedspherehq_2 "Animation Scale" (Variables|GasDisk|GetAnimation%20Scale))
          (Rendering|Material|SetScalarParameterValueonMaterials _invertedspherehq_2 "AnimExponent" (Variables|GasDisk|GetAnimExponent))
          (Rendering|Material|SetScalarParameterValueonMaterials _invertedspherehq_2 "Orbital Band Size" (Variables|GasDisk|GetOrbital%20Band%20Size))
          (Rendering|Material|SetScalarParameterValueonMaterials _invertedspherehq_2 "Fog Density" (Variables|GasDisk|GetFog%20Density))
          (Rendering|Material|SetScalarParameterValueonMaterials _invertedspherehq_2 "Fog Exponent" (Variables|GasDisk|GetFog%20Exponent))
          (Rendering|Material|SetScalarParameterValueonMaterials _invertedspherehq_2 "Fog Height" (Variables|GasDisk|GetFog%20Height))
          (Rendering|Material|SetScalarParameterValueonMaterials _invertedspherehq_2 "Light Bias" (Variables|GasDiskColors|GetLight%20Bias))
          (Rendering|Material|SetScalarParameterValueonMaterials _invertedspherehq_2 "Light Intensity" (Variables|GasDiskColors|GetLight%20Intensity))
          (Rendering|Material|SetScalarParameterValueonMaterials _invertedspherehq_2 "JitterAmount" (Variables|GasDiskColors|GetJitterAmount))
          (Rendering|Material|SetScalarParameterValueonMaterials _invertedspherehq_2 "ShadowDensity" (Variables|GasDiskColors|GetShadowDensity))
          (Rendering|Material|SetScalarParameterValueonMaterials _invertedspherehq_2 "ShadowSpread" (Variables|GasDiskColors|GetShadowSpread))
          (Rendering|Material|SetScalarParameterValueonMaterials _invertedspherehq_2 "ShadowStepSize" (Variables|GasDiskColors|GetShadowStepSize))
          (Rendering|Material|SetVectorParameterValueonMaterials _invertedspherehq_2 "LightColor" (Math|Conversions|ToVector(LinearColor) (Variables|GasDiskColors|GetLightColor)))
          (Rendering|Material|SetVectorParameterValueonMaterials _invertedspherehq_2 "ShadowColor" (Math|Conversions|ToVector(LinearColor) (Variables|GasDiskColors|GetShadowColor))))
        (:then_1
          ;[1 1 1] Collapse_Function
          (if (Variables|Matter&Mass|GetCollapse?)
            (while (>= (Variables|Matter&Mass|GetMass) 1e+02)
              (Variables|Matter&Mass|SetMass 1.0))
            (Rendering|Material|SetScalarParameterValueonMaterials _invertedspherehq "GravityMass" (Variables|Matter&Mass|GetGravitationalLensing))
            ;;[1 1 1] Set this Manually if you want Grav. Lensing with Star
            (Transformation|SetRelativeScale3D (Variables|Default|GetStar_Mesh) "0, 0, 0")
            (Rendering|Material|SetScalarParameterValueonMaterials (Variables|Default|GetInvertedSphereHQ) "Mass" (Variables|Matter&Mass|GetMass))
            (else
              ;[1 1 1] Star_Control
              (Variables|Matter&Mass|SetMass 1e+02)
              (Rendering|Material|SetScalarParameterValueonMaterials _invertedspherehq "GravityMass" 0.0)
              (Transformation|SetRelativeScale3D (Variables|Default|GetStar_Mesh) (Math|Conversions|ToVector(Float) _starsize))
              (Rendering|Material|SetScalarParameterValueonMaterials (Variables|Default|GetInvertedSphereHQ) "Mass" (/ (* (Variables|Matter&Mass|GetMass) _starsize) 2.0))
              (Niagara|SetNiagaraVariable(Float) (Variables|Default|GetNS_Sun_Rays) "Scale" (* _starsize 4.5e+06))
              (Niagara|SetNiagaraVariable(LinearColor) (Variables|Default|GetNS_Sun_Rays) "AtmosphereColor" (Variables|StarColors|GetAtmosphere%20Color)))))
        (:then_2
          ;[1 1 1] Set_Textures
          (Rendering|Material|SetScalarParameterValueonMaterials (Variables|Default|GetInvertedSphereHQ) "Celestial Disk Brightness" (Variables|CelestialBackground|GetCelestial%20Disk%20Exponent_Brightness))
          (Rendering|Material|SetScalarParameterValueonMaterials (Variables|Default|GetInvertedSphereHQ) "Celestial Disk Exponent" (Variables|CelestialBackground|GetCelestial%20Disk%20Exponent))
          (Rendering|Material|SetTextureParameterValue _returnvalue "Flow_map" (Variables|CelestialTextures|GetFlow%20Map))
          (Rendering|Material|SetTextureParameterValue _returnvalue "T_Color" (Variables|CelestialTextures|GetCubemap%20Texture))
          (Rendering|Material|SetTextureParameterValue _returnvalue "T_Alpha" (Variables|CelestialTextures|GetCubemap%20Texture%20Alpha))
          (Rendering|Material|SetTextureParameterValue _returnvalue "T_Color_Extra_Cubemap" (Variables|CelestialTextures|GetExtra%20Cubemap%20Texture))
          (Rendering|Material|SetTextureParameterValue _returnvalue "T_Alpha_Extra_Cubemap" (Variables|CelestialTextures|GetExtra%20Cubemap%20Texture%20Alpha))
          (Rendering|Material|SetTextureParameterValue _returnvalue "T_Stars_Near" (Variables|CelestialTextures|GetNearby%20Stars))
          (Rendering|Material|SetTextureParameterValue _returnvalue "T_Stars_Far" (Variables|CelestialTextures|GetFaraway%20Stars))
          ;[1 1 1] Star_Control
          (Rendering|Material|SetScalarParameterValueonMaterials _invertedspherehq_3 "Near_Stars_Desaturation" (Variables|CelestialStarControl|GetNearby%20Stars%20Desaturation))
          (Rendering|Material|SetScalarParameterValueonMaterials _invertedspherehq_3 "Far_Stars_Desaturation" (Variables|CelestialStarControl|GetFaraway%20Stars%20Desaturation))
          (Rendering|Material|SetScalarParameterValueonMaterials _invertedspherehq_3 "Near_Stars_intensity" (Variables|CelestialStarControl|GetNearby%20Stars%20Intensity))
          (Rendering|Material|SetScalarParameterValueonMaterials _invertedspherehq_3 "Far_Stars_intensity" (Variables|CelestialStarControl|GetFaraway%20Stars%20Intensity))
          ;[1 1 1] Color_Control
          (Rendering|Material|SetScalarParameterValueonMaterials _invertedspherehq_3 "Red_Level" (Variables|CelestialBackground|GetRed%20Level))
          (Rendering|Material|SetScalarParameterValueonMaterials _invertedspherehq_3 "Green_Level" (Variables|CelestialBackground|GetGreen%20Level))
          (Rendering|Material|SetScalarParameterValueonMaterials _invertedspherehq_3 "Blue_Level" (Variables|CelestialBackground|GetBlue%20Level))
          ;[1 1 1] Color_Control_Extra_Cubemap
          (Rendering|Material|SetScalarParameterValueonMaterials _invertedspherehq_3 "Red_Level_Extra_Cubemap" (Variables|CelestialBackground|GetExtra%20Cubemap%20Red%20Level))
          (Rendering|Material|SetScalarParameterValueonMaterials _invertedspherehq_3 "Green_Level_Extra_Cubemap" (Variables|CelestialBackground|GetExtra%20Cubemap%20Green%20Level))
          (Rendering|Material|SetScalarParameterValueonMaterials _invertedspherehq_3 "Blue_Level_Extra_Cubemap" (Variables|CelestialBackground|GetExtra%20Cubemap%20Blue%20Level))
          ;[1 1 1] Visibility_Control
          (Rendering|Material|SetScalarParameterValueonMaterials _invertedspherehq_3 "Power" (Variables|CelestialBackground|GetPower%20Level))
          (Rendering|Material|SetScalarParameterValueonMaterials _invertedspherehq_3 "Saturation" (Variables|CelestialBackground|GetSaturation))
          (Rendering|Material|SetVectorParameterValueonMaterials _invertedspherehq_3 "Flow_Direction" (Variables|CelestialBackground|GetFlow%20Movement%20Coordinates))
          (Rendering|Material|SetScalarParameterValueonMaterials _invertedspherehq_3 "Sun_Mask_Intensity" (Variables|CelestialBackground|GetSun%20Mask%20Intensity))
          ;[1 1 1] Visibility_Extra_Cubemap
          (Rendering|Material|SetScalarParameterValueonMaterials _invertedspherehq_3 "Saturation_Extra_Cubemap" (Variables|CelestialBackground|GetExtra%20Cubemap%20Saturation))
          (Rendering|Material|SetScalarParameterValueonMaterials _invertedspherehq_3 "Power_Extra_Cubemap" (Variables|CelestialBackground|GetExtra%20Cubemap%20Power%20Level))
          (Rendering|Material|SetScalarParameterValueonMaterials _invertedspherehq_3 "Cubemap_Rotation" (Variables|CelestialBackground|GetExtra%20Cubemap%20Rotation)))))
    (:then_1
      (Rendering|Material|CreateDynamicMaterialInstance (Variables|Default|GetStar_Mesh) 0 "/Game/Z_Add-Ons/Space_Construction/Planet_System/Materials/Star/M_Star_Solar_Inst.M_Star_Solar_Inst" "None" :!class /Script/Engine.PrimitiveComponent)
      ;[1 1 1] Sun Surface
      (Rendering|Material|SetScalarParameterValueonMaterials _star_mesh "Brightness" (Variables|StarSurface|GetStar%20Brightness))
      (Rendering|Material|SetScalarParameterValueonMaterials _star_mesh "Brightness Intensity" (Variables|StarSurface|GetBrightness%20Intensity))
      (Rendering|Material|SetScalarParameterValueonMaterials _star_mesh "Brightness Thickness" (Variables|StarSurface|GetBrightness%20Thickness))
      (Rendering|Material|SetScalarParameterValueonMaterials _star_mesh "Cell Edge Brightness" (Variables|StarSurface|GetCell%20Edge%20Brightness))
      (Rendering|Material|SetScalarParameterValueonMaterials _star_mesh "Cracks Amount" (Variables|StarSurface|GetCracks%20Amount))
      (Rendering|Material|SetScalarParameterValueonMaterials _star_mesh "Cracks Distortion" (Variables|StarSurface|GetCracks%20Distortion))
      (Rendering|Material|SetScalarParameterValueonMaterials _star_mesh "Cracks Intensity" (Variables|StarSurface|GetCracks%20Intensity))
      (Rendering|Material|SetScalarParameterValueonMaterials _star_mesh "Cracks Size" (Variables|StarSurface|GetCracks%20Size))
      ;[1 1 1] Flare Coverage
      (Rendering|Material|SetScalarParameterValueonMaterials _star_mesh "Dark Filaments Contrast" (Variables|FlareCoverage|GetDark%20Filaments%20Contrast))
      (Rendering|Material|SetScalarParameterValueonMaterials _star_mesh "Dark Filaments Coverage" (Variables|FlareCoverage|GetDark%20Filaments%20Coverage))
      (Rendering|Material|SetScalarParameterValueonMaterials _star_mesh "Deep Cell Edge Brightness" (Variables|FlareCoverage|GetDeep%20Cell%20Edge%20Brightness))
      (Rendering|Material|SetScalarParameterValueonMaterials _star_mesh "Distance Luminosity" (Variables|FlareCoverage|GetDistance%20Luminosity))
      (Rendering|Material|SetScalarParameterValueonMaterials _star_mesh "Distortion 2" (Variables|FlareCoverage|GetDistortion%202))
      (Rendering|Material|SetScalarParameterValueonMaterials _star_mesh "Distortion 3" (Variables|FlareCoverage|GetDistortion%203))
      (Rendering|Material|SetScalarParameterValueonMaterials _star_mesh "Filaments Amount" (Variables|FlareCoverage|GetFilaments%20Amount))
      (Rendering|Material|SetScalarParameterValueonMaterials _star_mesh "Filaments Position" (Variables|FlareCoverage|GetFilaments%20Position))
      (Rendering|Material|SetScalarParameterValueonMaterials _star_mesh "Flares Amount" (Variables|FlareCoverage|GetFlares%20Amount))
      (Rendering|Material|SetScalarParameterValueonMaterials _star_mesh "Flares Brightness" (Variables|FlareCoverage|GetFlares%20Brightness))
      (Rendering|Material|SetScalarParameterValueonMaterials _star_mesh "Flares Coverage" (Variables|FlareCoverage|GetFlares%20Coverage))
      ;[1 1 1] Macro/Micro Cells
      (Rendering|Material|SetScalarParameterValueonMaterials _star_mesh "Large Cells Brightness" (Variables|Macro/MicroCells|GetLarge%20Cells%20Brightness))
      (Rendering|Material|SetScalarParameterValueonMaterials _star_mesh "Large Cells Elevation" (Variables|Macro/MicroCells|GetLarge%20Cells%20Elevation))
      (Rendering|Material|SetScalarParameterValueonMaterials _star_mesh "Macro Cell Distortion_01" (Variables|Macro/MicroCells|GetMacro%20Cell%20Distortion_01))
      (Rendering|Material|SetScalarParameterValueonMaterials _star_mesh "Macro Cell Distortion_02" (Variables|Macro/MicroCells|GetMacro%20Cell%20Distortion_02))
      (Rendering|Material|SetScalarParameterValueonMaterials _star_mesh "Macro Cells Amount" (Variables|Macro/MicroCells|GetMacro%20Cells%20Amount))
      (Rendering|Material|SetScalarParameterValueonMaterials _star_mesh "Plates Coverage" (Variables|Macro/MicroCells|GetPlates%20Coverage))
      (Rendering|Material|SetScalarParameterValueonMaterials _star_mesh "Small Cells Brightness" (Variables|Macro/MicroCells|GetSmall%20Cells%20Brightness))
      (Rendering|Material|SetScalarParameterValueonMaterials _star_mesh "Small Cells Distortion" (Variables|Macro/MicroCells|GetSmall%20Cells%20Distortion))
      (Rendering|Material|SetScalarParameterValueonMaterials _star_mesh "Turbolence Speed" (Variables|Macro/MicroCells|GetTurbolence%20Speed))
      ;[1 1 1] Star Colors
      (Rendering|Material|SetVectorParameterValueonMaterials _star_mesh "Atmosphere Color" (Math|Conversions|ToVector(LinearColor) (Variables|StarColors|GetAtmosphere%20Fresnel%20Color)))
      (Rendering|Material|SetVectorParameterValueonMaterials _star_mesh "Color - High Altitude" (Math|Conversions|ToVector(LinearColor) (Variables|StarColors|GetColor%20Top%20Altitude)))
      (Rendering|Material|SetVectorParameterValueonMaterials _star_mesh "Color - Low Altitude" (Math|Conversions|ToVector(LinearColor) (Variables|StarColors|GetColor%20Bottom%20Altitude)))
      (Rendering|Material|SetVectorParameterValueonMaterials _star_mesh "Color Dark Flames" (Math|Conversions|ToVector(LinearColor) (Variables|StarColors|GetColor%20Dark%20Flames)))
      (Rendering|Material|SetVectorParameterValueonMaterials _star_mesh "Color Flares" (Math|Conversions|ToVector(LinearColor) (Variables|StarColors|GetColor%20Flares)))
      (Rendering|Material|SetVectorParameterValueonMaterials _star_mesh "Small Cells Color" (Math|Conversions|ToVector(LinearColor) (Variables|StarColors|GetSmall%20Cell%20Color)))
      ;[1 1 1] Star Atmopshere
      (Rendering|Material|SetScalarParameterValueonMaterials _star_mesh "Atmos_Haze Edge" (Variables|StarAtmosphere|GetAtmosphere%20Haze%20Edge))
      (Rendering|Material|SetScalarParameterValueonMaterials _star_mesh "Atmos_Haze Intensity" (Variables|StarAtmosphere|GetAtmosphere%20Haze%20Intensity))
      (Rendering|Material|SetScalarParameterValueonMaterials _star_mesh "Atmosphere Edge" (Variables|StarAtmosphere|GetAtmosphere%20Edge))
      (Rendering|Material|SetScalarParameterValueonMaterials _star_mesh "Atmosphere Intensity" (Variables|StarAtmosphere|GetAtmosphere%20Intensity))
      (Rendering|Material|SetScalarParameterValueonMaterials _star_mesh "Bright Zones Amount" (Variables|StarAtmosphere|GetBright%20Zones%20Amount))
      (Rendering|Material|SetScalarParameterValueonMaterials _star_mesh "Bright Zones Distortion" (Variables|StarAtmosphere|GetBright%20Zones%20Distortion)))))