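; Swimmable water volume actor that puts Rayman_BP into swimming, sized by WaterSize in the construction script.
; Overlap with SwimDetect switches movement to Swimming, clears ledge-grab and hover states, and caps swim height at the Plane's Z.
; UnderwaterDetect overlaps toggle Underwater and call CheckUnderwater on entry and exit.
; SwimDetect leaving does nothing, as the logic restoring Walking is disconnected.
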(event OnComponentBeginOverlap(WaterVolume)
  (params (OverlappedComponent :type Primitive%20Component%20Object%20Reference) (OtherActor :type Actor%20Object%20Reference) (OtherComp :type Primitive%20Component%20Object%20Reference) (OtherBodyIndex :type Integer) (bFromSweep :type Boolean) (SweepResult :type Hit%20Result%20Structure%20%28by%20ref%29))
  (bind _asrayman_bp (Utilities|Casting|CastToRayman_BP OtherActor))
  (if (== (Variables|/Game/Z_LumenEngine/Characters/Rayman/Rayman_BP.Rayman_BP_C|GetSwimDetect _asrayman_bp) OtherComp)
    (Utilities|Time|ClearTimerbyFunctionName _asrayman_bp "GrabLedge")
    (Pawn|Components|CharacterMovement|SetMovementMode (Variables|/Script/Engine.Character|GetCharacterMovement _asrayman_bp) "MOVE_Swimming" 0)
    (Variables|/Game/Z_LumenEngine/Characters/Rayman/Rayman_BP.Rayman_BP_C|SetGrabbingLedge _asrayman_bp false)
    (Variables|/Game/Z_LumenEngine/Characters/Rayman/Rayman_BP.Rayman_BP_C|SetHovering _asrayman_bp false)
    (Variables|/Game/Z_LumenEngine/Characters/Rayman/Rayman_BP.Rayman_BP_C|SetSwimming _asrayman_bp true)
    (Variables|/Script/Engine.PhysicsVolume|SetbWaterVolume (Class|MovementComponent|GetPhysicsVolume (Variables|/Script/Engine.Character|GetCharacterMovement _asrayman_bp)) true)
    (Variables|/Script/Engine.CharacterMovementComponent|SetRotationRate (Variables|/Script/Engine.Character|GetCharacterMovement _asrayman_bp) "360.000000,360.000000,360.000000")
    (Variables|/Game/Z_LumenEngine/Characters/Rayman/Rayman_BP.Rayman_BP_C|SetMaxSwimmingHeight _asrayman_bp (.z (Transformation|GetWorldLocation (Variables|Default|GetPlane))))
    (Development|PrintString "Hello")
    (elif (== (Variables|/Game/Z_LumenEngine/Characters/Rayman/Rayman_BP.Rayman_BP_C|GetUnderwaterDetect _asrayman_bp) OtherComp)
      (Variables|/Game/Z_LumenEngine/Characters/Rayman/Rayman_BP.Rayman_BP_C|SetUnderwater _asrayman_bp true)
      (Default|CheckUnderwater _asrayman_bp))))

(event OnComponentEndOverlap(WaterVolume)
  (params (OverlappedComponent :type Primitive%20Component%20Object%20Reference) (OtherActor :type Actor%20Object%20Reference) (OtherComp :type Primitive%20Component%20Object%20Reference) (OtherBodyIndex :type Integer))
  (bind _asrayman_bp (Utilities|Casting|CastToRayman_BP OtherActor))
  (if (not (== (Variables|/Game/Z_LumenEngine/Characters/Rayman/Rayman_BP.Rayman_BP_C|GetSwimDetect _asrayman_bp) OtherComp))
    (if (== (Variables|/Game/Z_LumenEngine/Characters/Rayman/Rayman_BP.Rayman_BP_C|GetUnderwaterDetect _asrayman_bp) OtherComp)
      (Variables|/Game/Z_LumenEngine/Characters/Rayman/Rayman_BP.Rayman_BP_C|SetUnderwater _asrayman_bp false)
      (Default|CheckUnderwater _asrayman_bp))))

(fn ConstructionScript
  (Transformation|SetWorldScale3D (Variables|Default|GetWaterVolume) (Variables|Default|GetWaterSize)))