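; SaveGameTrigger_BP is a trigger volume that saves progress when Rayman enters it in a linear game.
; It destroys itself on BeginPlay when the game instance is not in LinearGame mode.
; The first overlap by Rayman_BP calls the game instance's SaveGame with its trigger ID and current BGM, enabling story-mode load and saving the current level.
; The construction script sizes the box and displays the ID as text.
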(event OnComponentBeginOverlap(Box)
  (params (OverlappedComponent :type Primitive%20Component%20Object%20Reference) (OtherActor :type Actor%20Object%20Reference) (OtherComp :type Primitive%20Component%20Object%20Reference) (OtherBodyIndex :type Integer) (bFromSweep :type Boolean) (SweepResult :type Hit%20Result%20Structure%20%28by%20ref%29))
  (Utilities|Casting|CastToRayman_BP OtherActor)
  (Utilities|FlowControl|DoOnce false
    (:Completed
      (Default|SaveGame (.AsMain%20Game%20Instance (Utilities|Casting|CastToMain_GameInstance (Game|GetGameInstance))) (Variables|Default|GetSave%20Game%20Trigger%20ID) true true (Variables|Default|GetCurrentBGM)))))

(event EventBeginPlay
  (if (not (Variables|/Game/Main_GameInstance.Main_GameInstance_C|GetLinearGame (.AsMain%20Game%20Instance (Utilities|Casting|CastToMain_GameInstance (Game|GetGameInstance)))))
    (Actor|DestroyActor)))

(fn ConstructionScript
  (Components|Box|SetBoxExtent (Variables|Default|GetBox) (Variables|Default|GetTriggerSize) true)
  (Rendering|Components|TextRender|SetText (Variables|Default|GetTextRender1) (Utilities|Text|ToText(Integer) (Variables|Default|GetSave%20Game%20Trigger%20ID))))