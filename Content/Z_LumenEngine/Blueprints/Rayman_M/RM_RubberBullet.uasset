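; Rubber bullet projectile for Rayman M that bounces off surfaces and leaves a trail of effects as it flies.
; A looping timer spawns a RubberBulletVFX_BP actor at the bullet's transform every tenth of a second.
; A FlipFlop on the projectile bounce event lets the first bounce pass, then on the second zeroes bounciness and makes the sphere ignore static and dynamic world collision.
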(event OnProjectileBounce(ProjectileMovement)
  (params (ImpactResult :type Hit%20Result%20Structure%20%28by%20ref%29) (ImpactVelocity :type Vector%20%28by%20ref%29 :default "0, 0, 0"))
  (Utilities|FlowControl|FlipFlop
    (:B
      (Variables|/Script/Engine.ProjectileMovementComponent|SetBounciness (Variables|Default|GetProjectileMovement) 0.0)
      (Collision|SetCollisionResponsetoChannel (Variables|Default|GetSphere) "ECC_WorldStatic" "ECR_Ignore")
      (Collision|SetCollisionResponsetoChannel (Variables|Default|GetSphere) "ECC_WorldDynamic" "ECR_Ignore"))))

(event Custom|SpawnParticle
  (bind _returnvalue (Transformation|GetActorTransform))
  (Game|SpawnActorfromClass "/Game/Z_LumenEngine/Blueprints/Rayman_M/RubberBulletVFX_BP.RubberBulletVFX_BP_C" (Math|Transform|MakeTransform (.location _returnvalue) (.rotation _returnvalue) "1.000000,1.000000,1.000000") "AlwaysSpawn" "OverrideRootScale" 0 0))

(event EventBeginPlay
  (|CallParentFunction)
  (Utilities|Time|SetTimerbyEvent (delegate Custom|SpawnParticle) 0.1 true))

(fn ConstructionScript
  (|CallParentFunction))