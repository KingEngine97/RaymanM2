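; RM_FakeGenerator is a hazard actor that damages Rayman on contact, its name suggesting a decoy generator.
; At BeginPlay it zeroes its rotation and lowers itself by a small fixed offset.
; When its Box overlaps a Rayman_BP other than its owner, it applies Damage, refreshes that player's battle HUD and destroys itself.
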(event OnComponentBeginOverlap(Box)
  (params (OverlappedComponent :type Primitive%20Component%20Object%20Reference) (OtherActor :type Actor%20Object%20Reference) (OtherComp :type Primitive%20Component%20Object%20Reference) (OtherBodyIndex :type Integer) (bFromSweep :type Boolean) (SweepResult :type Hit%20Result%20Structure%20%28by%20ref%29))
  (if (!= OtherActor (Components|GetOwner))
    (bind _asrayman_bp (Utilities|Casting|CastToRayman_BP OtherActor))
    (Default|CauseDamage _asrayman_bp (Variables|Default|GetDamage))
    (Default|UpdateHUD (Variables|/Game/Z_LumenEngine/HUD/InGame_W.InGame_W_C|GetInGame_Battle_W (Variables|/Game/Z_LumenEngine/Characters/Rayman/Rayman_BP.Rayman_BP_C|GetInGame_UI _asrayman_bp)))
    (Actor|DestroyActor)))

(event EventBeginPlay
  (bind _returnvalue (Transformation|GetActorLocation))
  (|CallParentFunction)
  (Transformation|SetActorRotation "0, 0, 0")
  (Transformation|SetActorLocation (Math|Vector|MakeVector (.x _returnvalue) (.y _returnvalue) (- (.z _returnvalue) 2e+01)) false false))

(fn ConstructionScript
  (|CallParentFunction))