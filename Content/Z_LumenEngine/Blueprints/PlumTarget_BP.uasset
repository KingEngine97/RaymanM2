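; PlumTarget_BP is a target that catches a plum released into its overlap sphere and holds it in place.
; On sphere overlap, it accepts only a Plum_BP that is not being grabbed, and a DoOnce limits this to a single plum.
; The plum is flagged as stuck, loses physics and overlap events, then snaps to the Arrow component's location and rotation while keeping its world scale.
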(event OnComponentBeginOverlap(Sphere)
  (params (OverlappedComponent :type Primitive%20Component%20Object%20Reference) (OtherActor :type Actor%20Object%20Reference) (OtherComp :type Primitive%20Component%20Object%20Reference) (OtherBodyIndex :type Integer) (bFromSweep :type Boolean) (SweepResult :type Hit%20Result%20Structure%20%28by%20ref%29))
  (bind _asplum_bp (Utilities|Casting|CastToPlum_BP OtherActor))
  (if (not (Variables|/Game/Z_LumenEngine/Blueprints/Plum_BP.Plum_BP_C|GetGrabbing _asplum_bp))
    (Utilities|FlowControl|DoOnce false
      (:Completed
        (Variables|/Game/Z_LumenEngine/Blueprints/Plum_BP.Plum_BP_C|SetStuckOnTarget _asplum_bp true)
        (Variables|/Script/Engine.PrimitiveComponent|SetbGenerateOverlapEvents (Variables|/Game/Z_LumenEngine/Blueprints/Plum_BP.Plum_BP_C|GetBox _asplum_bp) false)
        (Variables|/Script/Engine.PrimitiveComponent|SetbGenerateOverlapEvents (Variables|/Game/Z_LumenEngine/Blueprints/Plum_BP.Plum_BP_C|GetBox1 _asplum_bp) false)
        (Variables|/Script/Engine.PrimitiveComponent|SetbGenerateOverlapEvents (Variables|/Game/Z_LumenEngine/Blueprints/Plum_BP.Plum_BP_C|GetStaticMesh1 _asplum_bp) false)
        (Physics|SetSimulatePhysics (Variables|/Game/Z_LumenEngine/Blueprints/Plum_BP.Plum_BP_C|GetBox _asplum_bp) false)
        (Transformation|AttachComponentToComponent _asplum_bp (Variables|Default|GetArrow) "None" "SnapToTarget" "SnapToTarget" "KeepWorld" true)))))

(fn ConstructionScript)