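; RM_BuzzRocket is Rayman's rocket projectile, which takes over the player's view and registers itself on Rayman_BP while in flight.
; A timeline drives it forward, using sphere traces to detect impacts, while its collision sphere arms after a short delay.
; Sphere contacts deal damage and spawn explosion effects.
; Every impact triggers a one-time explosion that damages a single traced actor, clears Rayman's rocket state, restores the view and destroys the rocket.
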(event OnComponentBeginOverlap(Sphere)
  (params (OverlappedComponent :type Primitive%20Component%20Object%20Reference) (OtherActor :type Actor%20Object%20Reference) (OtherComp :type Primitive%20Component%20Object%20Reference) (OtherBodyIndex :type Integer) (bFromSweep :type Boolean) (SweepResult :type Hit%20Result%20Structure%20%28by%20ref%29))
  (bind _returnvalue (Transformation|GetActorLocation))
  (bind _returnvalue_2 (Transformation|GetActorLocation))
  (bind _returnvalue_3 (Transformation|GetActorLocation))
  (if (!= OtherActor (Game|GetPlayerCharacter 0))
    (Class|RaymanInterface|CauseDamage(Message) OtherActor 40)
    (CallFunction|ExplodeRocket)
    (Niagara|SpawnSystematLocation "/Game/AdvancedMagicFX13/Particles/Niagara/NS_ky_explosion1.NS_ky_explosion1" _returnvalue_2 "0, 0, 0" "0.500000,0.500000,0.500000")
    (Audio|SpawnSoundatLocation "/Game/Audio/SFX/_extracted/4290606.4290606" _returnvalue_2 "0, 0, 0" 1.0 1.0 0.0 "/Game/Audio/LowAttenuation.LowAttenuation" 0)
    (bind _newtrack_0 (Timeline|Timeline_0 Stop)
      (:Update
        (Transformation|AddActorWorldOffset (* (Transformation|GetActorForwardVector) (* 1e+03 (Utilities|Time|GetWorldDeltaSeconds))))
        (bind _returnvalue_4 (Collision|SphereTraceByChannel _returnvalue _returnvalue 2e+01 "TraceTypeQuery1" false 0 "None"))
        (if _returnvalue_4
          (CallFunction|ExplodeRocket :!label _label)
          (Timeline|Timeline_0 Stop)
          (else
            (bind _returnvalue_5 (Collision|SphereTraceByChannel _returnvalue_3 _returnvalue_3 2e+01 "TraceTypeQuery4" false 0 "None"))
            (if _returnvalue_5
              (goto _label))))))))

(event OnComponentHit(Sphere)
  (params (HitComponent :type Primitive%20Component%20Object%20Reference) (OtherActor :type Actor%20Object%20Reference) (OtherComp :type Primitive%20Component%20Object%20Reference) (NormalImpulse :type Vector :default "0, 0, 0") (Hit :type Hit%20Result%20Structure%20%28by%20ref%29))
  (bind _returnvalue (Transformation|GetActorLocation))
  (bind _returnvalue_2 (Transformation|GetActorLocation))
  (bind _returnvalue_3 (Transformation|GetActorLocation))
  (if (!= OtherActor (Game|GetPlayerCharacter 0))
    (Class|RaymanInterface|CauseDamage(Message) (stale OnComponentBeginOverlap(Sphere) OtherActor) 40)
    (CallFunction|ExplodeRocket)
    (Niagara|SpawnSystematLocation "/Game/AdvancedMagicFX13/Particles/Niagara/NS_ky_explosion1.NS_ky_explosion1" _returnvalue_2 "0, 0, 0" "0.500000,0.500000,0.500000")
    (Audio|SpawnSoundatLocation "/Game/Audio/SFX/_extracted/4290606.4290606" _returnvalue_2 "0, 0, 0" 1.0 1.0 0.0 "/Game/Audio/LowAttenuation.LowAttenuation" 0)
    (bind _newtrack_0 (Timeline|Timeline_0 Stop)
      (:Update
        (Transformation|AddActorWorldOffset (* (Transformation|GetActorForwardVector) (* 1e+03 (Utilities|Time|GetWorldDeltaSeconds))))
        (bind _returnvalue_4 (Collision|SphereTraceByChannel _returnvalue _returnvalue 2e+01 "TraceTypeQuery1" false 0 "None"))
        (if _returnvalue_4
          (CallFunction|ExplodeRocket :!label _label)
          (Timeline|Timeline_0 Stop)
          (else
            (bind _returnvalue_5 (Collision|SphereTraceByChannel _returnvalue_3 _returnvalue_3 2e+01 "TraceTypeQuery4" false 0 "None"))
            (if _returnvalue_5
              (goto _label))))))))

(event Custom|ExplodeRocket
  (bind _returnvalue (Transformation|GetActorLocation))
  (bind _returnvalue_2 (Game|GetPlayerCharacter 0))
  (bind _sphere (Variables|Default|GetSphere))
  (bind _asrayman_bp (Utilities|Casting|CastToRayman_BP _returnvalue_2))
  (Utilities|FlowControl|DoOnce false
    (:Completed
      (Collision|SetCollisionEnabled _sphere "NoCollision")
      (Variables|/Script/Engine.PrimitiveComponent|SetbGenerateOverlapEvents _sphere false)
      (bind (_outhit _returnvalue_3) (Collision|SphereTraceByChannel _returnvalue _returnvalue 125.0 "TraceTypeQuery4" false 0 "ForDuration"))
      (if _returnvalue_3
        (Class|RaymanInterface|CauseDamage(Message) (.HitActor (Collision|BreakHitResult _outhit)) (Variables|Default|GetDamage)))
      (Variables|/Game/Characters/Rayman/Rayman_BP.Rayman_BP_C|SetRocketAiming _asrayman_bp false)
      (Variables|/Game/Characters/Rayman/Rayman_BP.Rayman_BP_C|SetRocketControlling _asrayman_bp false)
      (Variables|/Game/Characters/Rayman/Rayman_BP.Rayman_BP_C|SetBuzzRocket _asrayman_bp 0)
      (Utilities|FlowControl|Delay 0.5)
      (Game|Player|SetViewTargetwithBlend (Game|GetPlayerController 0) (Game|GetPlayerCharacter 0) 0.0 "VTBlend_Linear" 0.0 false)
      (Components|Activation|Deactivate (Variables|Default|GetCamera))
      (Actor|DestroyActor))))

(event EventBeginPlay
  (bind _returnvalue (Transformation|GetActorLocation))
  (bind _returnvalue_2 (Game|GetPlayerCharacter 0))
  (bind _returnvalue_3 (Transformation|GetActorLocation))
  (bind _sphere (Variables|Default|GetSphere))
  (bind _asrayman_bp (Utilities|Casting|CastToRayman_BP _returnvalue_2))
  (|CallParentFunction)
  (Variables|/Game/Characters/Rayman/Rayman_BP.Rayman_BP_C|SetBuzzRocket _asrayman_bp self)
  (Variables|/Game/Characters/Rayman/Rayman_BP.Rayman_BP_C|SetRocketAiming _asrayman_bp true)
  (Components|Activation|Activate (Variables|Default|GetCamera) false)
  (Game|Player|SetViewTargetwithBlend (Game|GetPlayerController 0) self 0.0 "VTBlend_Linear" 0.0 false)
  (Audio|SpawnSoundatLocation "/Game/Audio/SFX/_extracted/10392548.10392548" "0, 0, 0" "0, 0, 0" 1.0 1.0 0.0 "/Game/Audio/LowAttenuation.LowAttenuation" 0)
  (Utilities|FlowControl|Sequence
    (:then_0
      (bind _newtrack_0 (Timeline|Timeline_0 PlayFromStart)
        (:Update
          (Transformation|AddActorWorldOffset (* (Transformation|GetActorForwardVector) (* 1e+03 (Utilities|Time|GetWorldDeltaSeconds))))
          (bind _returnvalue_4 (Collision|SphereTraceByChannel _returnvalue _returnvalue 2e+01 "TraceTypeQuery1" false 0 "None"))
          (if _returnvalue_4
            (CallFunction|ExplodeRocket :!label _label)
            (Timeline|Timeline_0 Stop)
            (else
              (bind _returnvalue_5 (Collision|SphereTraceByChannel _returnvalue_3 _returnvalue_3 2e+01 "TraceTypeQuery4" false 0 "None"))
              (if _returnvalue_5
                (goto _label)))))))
    (:then_1
      (Utilities|FlowControl|Delay 0.5)
      (Collision|SetCollisionEnabled _sphere "QueryAndPhysics")
      (Variables|/Script/Engine.PrimitiveComponent|SetbGenerateOverlapEvents _sphere true))))

(fn ConstructionScript
  (|CallParentFunction))