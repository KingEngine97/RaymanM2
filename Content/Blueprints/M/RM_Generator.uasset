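; RM_Generator is a weapon pickup actor that grants a weapon to Rayman_BP characters.
; On BeginPlay it can optionally pick a random weapon from the battle weapon set.
; When a Rayman overlaps its box, it sets that character's current weapon and matching starting ammo, refreshes the battle HUD, and destroys itself.
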(event OnComponentBeginOverlap(Box)
  (params (OverlappedComponent :type Primitive%20Component%20Object%20Reference) (OtherActor :type Actor%20Object%20Reference) (OtherComp :type Primitive%20Component%20Object%20Reference) (OtherBodyIndex :type Integer) (bFromSweep :type Boolean) (SweepResult :type Hit%20Result%20Structure%20%28by%20ref%29))
  (bind _asrayman_bp (Utilities|Casting|CastToRayman_BP OtherActor))
  (bind _output_get (Variables|/Game/Characters/Rayman/Rayman_BP.Rayman_BP_C|SetCurrentWeapon _asrayman_bp (Variables|Default|GetWeapon)))
  (Variables|/Game/Characters/Rayman/Rayman_BP.Rayman_BP_C|SetCurrentWeaponAmmo _asrayman_bp (Utilities|Select :Index _output_get :NewEnumerator0 0 :NewEnumerator1 1 :NewEnumerator2 1 :NewEnumerator3 1 :NewEnumerator4 1 :NewEnumerator5 1 :NewEnumerator6 9 :NewEnumerator7 3 :NewEnumerator8 3 :NewEnumerator9 3 :NewEnumerator10 3 :NewEnumerator11 3))
  (Default|UpdateHUD (Variables|/Game/HUD/InGame_W.InGame_W_C|GetInGame_Battle_W (Variables|/Game/Characters/Rayman/Rayman_BP.Rayman_BP_C|GetInGame_UI _asrayman_bp)))
  (Actor|DestroyActor))

(event EventBeginPlay
  (if (Variables|Default|GetRandomWeapon)
    (Variables|Default|SetWeapon (Utilities|Select :Index (Math|Random|RandomIntegerinRange 0 10) :Option%200 "NewEnumerator1" :Option%201 "NewEnumerator2" :Option%202 "NewEnumerator3" :Option%203 "NewEnumerator4" :Option%204 "NewEnumerator5" :Option%205 "NewEnumerator6" :Option%206 "NewEnumerator7" :Option%207 "NewEnumerator8" :Option%208 "NewEnumerator9" :Option%209 "NewEnumerator10" :Option%2010 "NewEnumerator11"))))

(fn ConstructionScript)