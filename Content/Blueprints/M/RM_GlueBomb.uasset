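; RM_GlueBomb is a projectile bomb that sticks to a Rayman_BP it touches and damages it after a countdown.
; Overlaps enable shortly after spawn, and a gate destroys the bomb after ten seconds unless a hit closes it.
; On overlap it snaps onto the character's BombSpline and stops moving.
; A DoOnce starts one sprite countdown, so later overlaps can move the bomb to another character without resetting the timer.
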(event OnComponentBeginOverlap(Sphere1)
  (params (OverlappedComponent :type Primitive%20Component%20Object%20Reference) (OtherActor :type Actor%20Object%20Reference) (OtherComp :type Primitive%20Component%20Object%20Reference) (OtherBodyIndex :type Integer) (bFromSweep :type Boolean) (SweepResult :type Hit%20Result%20Structure%20%28by%20ref%29))
  (bind _asrayman_bp (Utilities|Casting|CastToRayman_BP OtherActor))
  (Variables|Default|SetAttachedToActor _asrayman_bp)
  (Transformation|SetActorLocation (Spline|FindLocationClosesttoWorldLocation (Variables|/Game/Characters/Rayman/Rayman_BP.Rayman_BP_C|GetBombSpline _asrayman_bp) (Transformation|GetActorLocation) "World") false true)
  (Transformation|AttachComponentToComponent (Variables|/Game/Characters/Rayman/Rayman_BP.Rayman_BP_C|GetBombSpline _asrayman_bp) "None" "KeepWorld" "KeepWorld" "KeepWorld" true)
  (Components|Activation|Deactivate (Variables|Default|GetProjectileMovement))
  (Utilities|FlowControl|Sequence
    (:then_0
      (Utilities|FlowControl|Gate false) ; enters at Close
    )
    (:then_1
      (Utilities|FlowControl|DoOnce false
        (:Completed
          (Utilities|FlowControl|Sequence
            (:then_0
              (Utilities|FlowControl|Delay 1e+01)
              (Default|CauseDamage (Variables|Default|GetAttachedToActor) (Variables|Default|GetDamage))
              (Actor|DestroyActor))
            (:then_1
              (Rendering|Components|Sprite|SetSprite (Variables|Default|GetBillboard) (Utilities|Select :Index (Variables|Default|GetSecondsLeft) :Option%200 "/Game/Blueprints/M/GlueBomb/bombe_01.bombe_01" :Option%201 "/Game/Blueprints/M/GlueBomb/bombe_01.bombe_01" :Option%202 "/Game/Blueprints/M/GlueBomb/bombe_02.bombe_02" :Option%203 "/Game/Blueprints/M/GlueBomb/bombe_03.bombe_03" :Option%204 "/Game/Blueprints/M/GlueBomb/bombe_04.bombe_04" :Option%205 "/Game/Blueprints/M/GlueBomb/bombe_05.bombe_05" :Option%206 "/Game/Blueprints/M/GlueBomb/bombe_06.bombe_06" :Option%207 "/Game/Blueprints/M/GlueBomb/bombe_07.bombe_07" :Option%208 "/Game/Blueprints/M/GlueBomb/bombe_08.bombe_08" :Option%209 "/Game/Blueprints/M/GlueBomb/bombe_09.bombe_09" :Option%2010 "/Game/Blueprints/M/GlueBomb/bombe_10.bombe_10") :!label _label)
              (Utilities|FlowControl|Delay 1.0)
              (if (not (== (Variables|Default|GetSecondsLeft) 1))
                (Math|Integer|DecrementInt (Variables|Default|GetSecondsLeft)
                  (:%20%20
                    (goto _label)))))))))))

(event EventBeginPlay
  (|CallParentFunction)
  (Utilities|FlowControl|Delay 0.1)
  (Variables|/Script/Engine.PrimitiveComponent|SetbGenerateOverlapEvents (Variables|Default|GetSphere1) true)
  (Utilities|FlowControl|Delay 1e+01)
  (Utilities|FlowControl|Gate false
    (:Exit
      (Actor|DestroyActor))))

(fn ConstructionScript
  (|CallParentFunction))