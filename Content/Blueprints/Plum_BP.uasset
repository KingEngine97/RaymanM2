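; Plum actor that Rayman can pick up, carry, throw or ride, and that a RaymanHand or RocketLauncher hit releases into physics.
; Overlapping it at rest plays a grab montage and attaches it to a mesh socket, while a second box attaches Rayman as rider until JumpOff.
; Throw follows a distance-timed timeline arc to a "Plum"-tagged target, otherwise applies a forward impulse.
; DoOnce gates and overlap toggles rearm interactions unless StuckOnTarget is set.
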(event OnComponentBeginOverlap(StaticMesh1)
  (params (OverlappedComponent :type Primitive%20Component%20Object%20Reference) (OtherActor :type Actor%20Object%20Reference) (OtherComp :type Primitive%20Component%20Object%20Reference) (OtherBodyIndex :type Integer) (bFromSweep :type Boolean) (SweepResult :type Hit%20Result%20Structure%20%28by%20ref%29))
  (Utilities|Casting|CastToRaymanHand_BP OtherActor
    (:then
      _)
    (:CastFailed
      (Utilities|Casting|CastToRocketLauncher OtherActor)))
  (Utilities|FlowControl|DoOnce false
    (:Completed
      (Variables|/Script/Engine.PrimitiveComponent|SetbGenerateOverlapEvents (Variables|Default|GetBox) true)
      (Variables|/Script/Engine.PrimitiveComponent|SetbGenerateOverlapEvents (Variables|Default|GetBox1) true)
      (Variables|/Script/Engine.PrimitiveComponent|SetbGenerateOverlapEvents (Variables|Default|GetStaticMesh1) false)
      (Variables|Default|SetTags (Utilities|Array|MakeArray " "))
      (Physics|SetSimulatePhysics (Variables|Default|GetBox) true)
      (Utilities|FlowControl|Delay 1.0)
      (Class|PrimitiveComponent|SetLinearDamping (Variables|Default|GetBox) 0.5))))

(event OnComponentBeginOverlap(Box)
  (params (OverlappedComponent :type Primitive%20Component%20Object%20Reference) (OtherActor :type Actor%20Object%20Reference) (OtherComp :type Primitive%20Component%20Object%20Reference) (OtherBodyIndex :type Integer) (bFromSweep :type Boolean) (SweepResult :type Hit%20Result%20Structure%20%28by%20ref%29))
  (bind _returnvalue (Game|GetPlayerCharacter 0))
  (bind _asrayman_bp (Utilities|Casting|CastToRayman_BP OtherActor))
  (if (not (Variables|Default|GetStuckOnTarget))
    (if (Utilities|Operators|EqualEqual :A (Transformation|GetVelocity) :ErrorTolerance 5.0)
      (Utilities|FlowControl|DoOnce false
        (:Completed
          (Input|DisableInput _asrayman_bp (Game|GetPlayerController 0))
          (Transformation|SetActorRotation _returnvalue (Math|Rotator|MakeRotator 0.0 0.0 (.yaw (Math|Rotator|FindLookatRotation (Transformation|GetActorLocation _returnvalue) (Transformation|GetActorLocation)))))
          (Variables|Default|SetGrabbing true)
          (Variables|/Script/Engine.PrimitiveComponent|SetbGenerateOverlapEvents (Variables|Default|GetBox1) false)
          (Variables|/Game/Characters/Rayman/Rayman_BP.Rayman_BP_C|SetPlum _asrayman_bp self)
          (Pawn|Components|CharacterMovement|DisableMovement (Variables|/Script/Engine.Character|GetCharacterMovement _asrayman_bp))
          (Animation|PlayAnimMontage _asrayman_bp "/Game/Characters/Rayman/Animations/Montages/Rayman_Anim_OPENSPACE_MODEL_ARMATURE_OBJECT_OBJECT_Animation_47_Montage.Rayman_Anim_OPENSPACE_MODEL_ARMATURE_OBJECT_OBJECT_Animation_47_Montage" 1.0 "None")
          (Variables|/Game/Characters/Rayman/Rayman_BP.Rayman_BP_C|SetCarryingPlum _asrayman_bp true)
          (Physics|SetSimulatePhysics (Variables|Default|GetBox) false)
          (Collision|SetCollisionEnabled (Variables|Default|GetStaticMesh1) "NoCollision")
          (Utilities|FlowControl|Delay 0.35)
          (Transformation|AttachComponentToComponent (Variables|/Script/Engine.Character|GetMesh _asrayman_bp) "Channel-5_end" "SnapToTarget" "SnapToTarget" "KeepWorld" true)
          (Utilities|FlowControl|Delay 1.33)
          (Input|EnableInput _asrayman_bp (Game|GetPlayerController 0))
          (Pawn|Components|CharacterMovement|SetMovementMode (Variables|/Script/Engine.Character|GetCharacterMovement _asrayman_bp) "MOVE_Walking" 0)))
      (else
        (Variables|/Script/Engine.PrimitiveComponent|SetbGenerateOverlapEvents (Variables|Default|GetBox) false)
        (Utilities|FlowControl|Delay 0.05)
        (Variables|/Script/Engine.PrimitiveComponent|SetbGenerateOverlapEvents (Variables|Default|GetBox) true)))))

(event OnComponentBeginOverlap(Box1)
  (params (OverlappedComponent :type Primitive%20Component%20Object%20Reference) (OtherActor :type Actor%20Object%20Reference) (OtherComp :type Primitive%20Component%20Object%20Reference) (OtherBodyIndex :type Integer) (bFromSweep :type Boolean) (SweepResult :type Hit%20Result%20Structure%20%28by%20ref%29))
  (bind _asrayman_bp (Utilities|Casting|CastToRayman_BP OtherActor))
  (if (not (Variables|Default|GetStuckOnTarget))
    (Utilities|FlowControl|DoOnce false
      (:Completed
        (Variables|/Script/Engine.PrimitiveComponent|SetbGenerateOverlapEvents (Variables|Default|GetBox) false)
        (Variables|/Game/Characters/Rayman/Rayman_BP.Rayman_BP_C|SetRidingPlum _asrayman_bp true)
        (Variables|/Game/Characters/Rayman/Rayman_BP.Rayman_BP_C|SetPlum _asrayman_bp self)
        (Transformation|AttachActorToActor _asrayman_bp self "None" "KeepWorld" "KeepWorld" "KeepWorld" true)))))

(event Custom|Throw
  (bind _returnvalue (Game|GetPlayerCharacter 0))
  (bind _returnvalue_2 (Transformation|GetActorLocation))
  (Variables|Default|SetGrabbing false)
  (Collision|SetCollisionEnabled (Variables|Default|GetStaticMesh1) "QueryAndPhysics")
  (bind _asrayman_bp (Utilities|Casting|CastToRayman_BP (Game|GetPlayerCharacter 0)))
  (Utilities|IsValid (Variables|/Game/Characters/Rayman/Rayman_BP.Rayman_BP_C|GetTarget _asrayman_bp)
    (:Is%20Valid
      (if (Actor|ActorHasTag (Variables|/Game/Characters/Rayman/Rayman_BP.Rayman_BP_C|GetTarget _asrayman_bp) "Plum")
        (Utilities|FlowControl|Sequence
          (:then_0
            (Variables|Default|SetPlumStartLocation _returnvalue_2)
            (Variables|Default|SetTargetLocation (Transformation|GetWorldLocation (Variables|/Game/Blueprints/PlumTarget_BP.PlumTarget_BP_C|GetArrow (.AsPlum%20Target%20BP (Utilities|Casting|CastToPlumTarget_BP (Variables|/Game/Characters/Rayman/Rayman_BP.Rayman_BP_C|GetTarget _asrayman_bp))))))
            (Components|Timeline|SetPlayRate (Variables|Default|GetTimeline_0) (Math|Float|MapRangeClamped (Math|Vector|Distance(Vector) _returnvalue_2 (Transformation|GetWorldLocation (Variables|/Game/Blueprints/PlumTarget_BP.PlumTarget_BP_C|GetArrow (.AsPlum%20Target%20BP (Utilities|Casting|CastToPlumTarget_BP (Variables|/Game/Characters/Rayman/Rayman_BP.Rayman_BP_C|GetTarget _asrayman_bp)))))) 1e+02 8.5e+02 3.0 2.0))
            (bind _asrayman_bp_2 (Utilities|Casting|CastToRayman_BP (Game|GetPlayerCharacter 0)))
            (Variables|/Game/Characters/Rayman/Rayman_BP.Rayman_BP_C|SetCarryingPlum _asrayman_bp_2 false)
            (Variables|/Game/Characters/Rayman/Rayman_BP.Rayman_BP_C|SetTarget _asrayman_bp_2 0)
            (bind (_direction _newtrack_0 _newtrack_1) (Timeline|Timeline_0 PlayFromStart)
              (:Update
                (Transformation|SetActorLocation (Math|Vector|MakeVector (.X (Math|Vector|BreakVector (Math|Vector|Lerp(Vector) (Variables|Default|GetPlumStartLocation) (Variables|Default|GetTargetLocation) _newtrack_0))) (.Y (Math|Vector|BreakVector (Math|Vector|Lerp(Vector) (Variables|Default|GetPlumStartLocation) (Variables|Default|GetTargetLocation) _newtrack_0))) (+ (.Z (Math|Vector|BreakVector (Variables|Default|GetTargetLocation))) (Math|Float|Lerp 0.0 1e+02 _newtrack_1))) false true)
                (Transformation|SetActorRotation (Math|Rotator|Lerp(Rotator) "0, 0, 0" "0,360.000000, 0" _newtrack_0)))))
          (:then_1
            (Utilities|FlowControl|Delay 1.0 :!label _label)
            (bind _asrayman_bp_3 (Utilities|Casting|CastToRayman_BP (Game|GetPlayerCharacter 0)))
            (Variables|/Game/Characters/Rayman/Rayman_BP.Rayman_BP_C|SetCarryingPlum _asrayman_bp_3 false)
            (Variables|/Game/Characters/Rayman/Rayman_BP.Rayman_BP_C|SetTarget _asrayman_bp_3 0)
            (if (not (Variables|Default|GetStuckOnTarget))
              (Variables|/Script/Engine.PrimitiveComponent|SetbGenerateOverlapEvents (Variables|Default|GetBox1) true)
              (Utilities|FlowControl|DoOnce false) ; enters at Reset
            )))
        (else
          (Physics|SetSimulatePhysics (Variables|Default|GetBox) true :!label _label_2)
          (Physics|AddImpulse (Variables|Default|GetBox) (* (Transformation|GetActorForwardVector (Game|GetPlayerCharacter 0)) 8e+02) "None" true)
          (goto _label))))
    (:Is%20Not%20Valid
      (goto _label_2))))

(event Custom|JumpOff
  (Transformation|DetachFromActor (.AsRayman%20BP (Utilities|Casting|CastToRayman_BP (Game|GetPlayerCharacter 0))) "KeepWorld" "KeepWorld" "KeepWorld")
  (Utilities|FlowControl|Delay 1.0)
  (if (not (Variables|Default|GetStuckOnTarget))
    (Variables|/Script/Engine.PrimitiveComponent|SetbGenerateOverlapEvents (Variables|Default|GetBox) true)
    (Utilities|FlowControl|DoOnce false) ; enters at Reset
  ))

(fn ConstructionScript)