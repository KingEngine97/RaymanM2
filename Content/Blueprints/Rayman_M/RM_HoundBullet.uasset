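; RM_HoundBullet is a projectile Blueprint that tries to home in on a nearby Rayman_BP actor shortly after spawning.
; Half a second after BeginPlay, a debug-drawn multi-sphere trace around the bullet, ignoring its owner, gathers hits in a large radius.
; The hit with the smallest distance below the stored Distance becomes Target, whose root component, via a Rayman_BP cast, becomes the ProjectileMovement homing target.
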(event EventBeginPlay
  (bind _returnvalue (Transformation|GetActorLocation))
  (|CallParentFunction)
  (Utilities|FlowControl|Delay 0.5)
  (bind (_outhits _returnvalue_2) (Collision|MultiSphereTraceByChannel _returnvalue _returnvalue 2e+03 "TraceTypeQuery4" false (Utilities|Array|MakeArray (Components|GetOwner)) "ForDuration"))
  (if _returnvalue_2
    (for _array_element _outhits
      (if (< (.Distance (Collision|BreakHitResult _array_element)) (Variables|Default|GetDistance))
        (Variables|Default|SetDistance (.Distance (Collision|BreakHitResult _array_element)))
        (Variables|Default|SetTarget (.HitActor (Collision|BreakHitResult _array_element)))))
    (Variables|/Script/Engine.ProjectileMovementComponent|SetHomingTargetComponent (Variables|Default|GetProjectileMovement) (Variables|/Script/Engine.Actor|GetRootComponent (.AsRayman%20BP (Utilities|Casting|CastToRayman_BP (Variables|Default|GetTarget)))))))

(fn ConstructionScript
  (|CallParentFunction))