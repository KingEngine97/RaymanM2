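; RM_FireworkBullet is a firework projectile for Rayman that bursts on contact and deals damage in a small radius.
; A timeline started on BeginPlay runs a small sphere trace on the Visibility channel at the bullet's location each update.
; The first hit triggers a wider single-hit trace on another channel, sending CauseDamageMessage to the struck actor, then destroys the bullet.
; Both traces have debug drawing enabled, and a delayed-destroy branch is left unconnected.
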(event EventBeginPlay
  (bind _returnvalue (Transformation|GetActorLocation))
  (bind _returnvalue_2 (Transformation|GetActorLocation))
  (|CallParentFunction)
  (Timeline|Timeline_0 Play
    (:Update
      (bind _returnvalue_3 (Collision|SphereTraceByChannel _returnvalue_2 _returnvalue_2 2e+01 "TraceTypeQuery1" false 0 "ForOneFrame"))
      (if _returnvalue_3
        (Utilities|FlowControl|DoOnce false
          (:Completed
            (bind (_outhit _returnvalue_4) (Collision|SphereTraceByChannel _returnvalue _returnvalue 125.0 "TraceTypeQuery4" false 0 "ForDuration"))
            (if _returnvalue_4
              (Class|RaymanInterface|CauseDamage(Message) (.HitActor (Collision|BreakHitResult _outhit)) (Variables|Default|GetDamage)))
            (Components|DestroyComponent (Variables|Default|GetTimeline_0))
            (Utilities|IsValid self
              (:Is%20Valid
                (Actor|DestroyActor)))))))))

(fn ConstructionScript
  (|CallParentFunction))