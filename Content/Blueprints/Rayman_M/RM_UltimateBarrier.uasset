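; RM_UltimateBarrier is an actor that forms Rayman's ultimate barrier around the player.
; On BeginPlay it flags the barrier active on Rayman_BP, doubles its scale and snaps onto the player character.
; A timeline drives a debug-drawn, zero-length sphere trace each update, sending damage to the first actor hit, once only.
; That hit calls DestroyBarrier, which only clears the player's flag without destroying the actor.
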(event Custom|DestroyBarrier
  (bind _asrayman_bp (Utilities|Casting|CastToRayman_BP (Game|GetPlayerCharacter 0)))
  (Variables|/Game/Characters/Rayman/Rayman_BP.Rayman_BP_C|SetUltimateBarrierActive _asrayman_bp false))

(event EventBeginPlay
  (bind _returnvalue (Transformation|GetActorLocation))
  (|CallParentFunction)
  (bind _asrayman_bp (Utilities|Casting|CastToRayman_BP (Game|GetPlayerCharacter 0)))
  (Variables|/Game/Characters/Rayman/Rayman_BP.Rayman_BP_C|SetUltimateBarrierActive _asrayman_bp true)
  (Transformation|SetActorScale3D "2.000000,2.000000,2.000000")
  (Transformation|AttachActorToActor (Game|GetPlayerCharacter 0) "None" "SnapToTarget" "SnapToTarget" "KeepWorld" true)
  (Timeline|Timeline_0 Play
    (:Update
      (bind (_outhit _returnvalue_2) (Collision|SphereTraceByChannel _returnvalue _returnvalue 105.0 "TraceTypeQuery4" false (Utilities|Array|MakeArray (Components|GetOwner)) "ForOneFrame"))
      (if _returnvalue_2
        (Utilities|FlowControl|DoOnce false
          (:Completed
            (Class|RaymanInterface|CauseDamage(Message) (.HitActor (Collision|BreakHitResult _outhit)) (Variables|Default|GetDamage))
            (CallFunction|DestroyBarrier)))))))

(fn ConstructionScript
  (|CallParentFunction))