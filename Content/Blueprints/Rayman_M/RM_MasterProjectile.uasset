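; Master projectile Blueprint for the Rayman_M content that damages what it touches and then destroys itself.
; On BeginPlay it briefly delays before enabling overlap events on its Sphere, then self-destructs after TimeToDespawn unless that is zero.
; Sphere overlaps send CauseDamageMessage with Damage to any valid actor and destroy the projectile, unless IgnoreCharacterOverlapDamage is set.
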(event OnComponentBeginOverlap(Sphere)
  (params (OverlappedComponent :type Primitive%20Component%20Object%20Reference) (OtherActor :type Actor%20Object%20Reference) (OtherComp :type Primitive%20Component%20Object%20Reference) (OtherBodyIndex :type Integer) (bFromSweep :type Boolean) (SweepResult :type Hit%20Result%20Structure%20%28by%20ref%29))
  (if (not (Variables|Default|GetIgnoreCharacterOverlapDamage))
    (Utilities|IsValid OtherActor
      (:Is%20Valid
        (Class|RaymanInterface|CauseDamage(Message) OtherActor (Variables|Default|GetDamage))
        (Actor|DestroyActor)))))

(event EventBeginPlay
  (bind _timetodespawn (Variables|Default|GetTimeToDespawn))
  (Utilities|FlowControl|Delay 0.075)
  (Variables|/Script/Engine.PrimitiveComponent|SetbGenerateOverlapEvents (Variables|Default|GetSphere) true)
  (if (not (== _timetodespawn 0.0))
    (Utilities|FlowControl|Delay _timetodespawn)
    (Actor|DestroyActor)))

(fn ConstructionScript)