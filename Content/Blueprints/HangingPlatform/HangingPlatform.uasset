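; BP swing point (HangingPlatform) that BP_RaymanPawn grapples and hangs from on sphere overlap while Busy.
; RequiresCanPowerup selects the metal-lum or billboard look, cable material and Target tags, and gates grabbing on the player's power-up.
; A grab disables movement, lerps the player to an arrow, attaches them, then swings them with a looping-pivot timeline that tracks swing direction.
; StopHanging hides the cable, restores tags and resets the DoOnce gates.
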(event OnComponentBeginOverlap(Sphere)
  (params (OverlappedComponent :type Primitive%20Component%20Object%20Reference) (OtherActor :type Actor%20Object%20Reference) (OtherComp :type Primitive%20Component%20Object%20Reference) (OtherBodyIndex :type Integer) (bFromSweep :type Boolean) (SweepResult :type Hit%20Result%20Structure%20%28by%20ref%29))
  (bind _returnvalue (Game|GetPlayerCharacter 0))
  (bind _returnvalue_2 (Game|GetPlayerCharacter 0))
  (bind _asbp_rayman_pawn (Utilities|Casting|CastToBP_RaymanPawn _returnvalue))
  (bind _charactermovement (Variables|/Script/Engine.Character|GetCharacterMovement _returnvalue_2))
  (bind _asbp_rayman_pawn_2 (Utilities|Casting|CastToBP_RaymanPawn OtherActor))
  (if (Variables|/Game/Blueprint/Pawn/BP_RaymanPawn.BP_RaymanPawn_C|GetBusy _asbp_rayman_pawn_2)
    (if (Variables|Default|GetRequiresCanPowerup)
      (bind _asbp_rayman_pawn_3 (Utilities|Casting|CastToBP_RaymanPawn (Game|GetPlayerCharacter 0)))
      (if (Utilities|Enum|Equal(Enum) (Variables|/Game/Blueprint/Pawn/BP_RaymanPawn.BP_RaymanPawn_C|GetCurrentPowerUp _asbp_rayman_pawn_3) "NewEnumerator0")
        (Utilities|FlowControl|DoOnce false :!label _label
          (:Completed
            (Variables|Default|SetTags (Utilities|Array|MakeArray " " " "))
            (Transformation|SetWorldRotation (Variables|Default|GetSphere1) (Math|Rotator|MakeRotator 0.0 0.0 (.yaw (Math|Rotator|FindLookatRotation (Transformation|GetActorLocation (Game|GetPlayerCharacter 0)) (Transformation|GetActorLocation)))) false false)
            (Components|Timeline|SetPlaybackPosition (Variables|Default|GetTimeline_1) 0.0 false true)
            (bind _asbp_rayman_pawn_4 (Utilities|Casting|CastToBP_RaymanPawn (Game|Player|GetPlayerPawn 0)))
            (Default|JumpReleased _asbp_rayman_pawn_4)
            (if (Variables|Default|GetRequiresCanPowerup)
              (if (Utilities|Enum|Equal(Enum) (Variables|/Game/Blueprint/Pawn/BP_RaymanPawn.BP_RaymanPawn_C|GetCurrentPowerUp _asbp_rayman_pawn_4) "NewEnumerator0")
                (Utilities|IsValid (Variables|/Game/Blueprint/Pawn/BP_RaymanPawn.BP_RaymanPawn_C|GetSwinging%20Actor _asbp_rayman_pawn_4) :!label _label_2
                  (:Is%20Valid
                    (CallFunction|StopHanging))
                  (:Is%20Not%20Valid
                    _))
                (Variables|/Game/Blueprint/Pawn/BP_RaymanPawn.BP_RaymanPawn_C|SetSwinging%20Actor _asbp_rayman_pawn_4 self)
                (Utilities|FlowControl|DoOnce false
                  (:Completed
                    (if (Variables|Default|GetRequiresCanPowerup)
                      (Components|Animation|PlayAnimation (Variables|Default|Getgrabbable_metal_lum_for_hanging_anim1) "/Game/Blueprints/HangingPlatform/grabbable_metal_lum_for_hanging_anim1_Anim_OPENSPACE_MODEL_ARMATURE_OBJECT_OBJECT_Animation_4.grabbable_metal_lum_for_hanging_anim1_Anim_OPENSPACE_MODEL_ARMATURE_OBJECT_OBJECT_Animation_4" false)
                      (Utilities|FlowControl|Sequence
                        (:then_0
                          (Rendering|SetVisibility (Variables|Default|GetCable) true false :!label _label_3)
                          (Variables|/Game/Blueprint/Pawn/BP_RaymanPawn.BP_RaymanPawn_C|SetSwinging%20Actor _asbp_rayman_pawn self)
                          (Variables|/Game/Blueprint/Pawn/BP_RaymanPawn.BP_RaymanPawn_C|SetSwinging _asbp_rayman_pawn true)
                          (Pawn|Components|CharacterMovement|SetMovementMode _charactermovement "MOVE_Flying" 0)
                          (Pawn|Components|CharacterMovement|DisableMovement _charactermovement)
                          (Variables|Default|SetPlayerLocationStart (Transformation|GetActorLocation (Game|GetPlayerCharacter 0)))
                          (Transformation|SetRelativeRotation (Variables|Default|GetArrow) "-140.000000, 0, 0" false false)
                          (bind _newtrack_0 (Timeline|Timeline_2 PlayFromStart)
                            (:Update
                              (Transformation|SetActorLocation (Game|GetPlayerCharacter 0) (Math|Vector|Lerp(Vector) (Variables|Default|GetPlayerLocationStart) (Transformation|GetWorldLocation (Variables|Default|GetArrow3)) _newtrack_0) false true))
                            (:Finished
                              (Transformation|AttachComponentToComponent _returnvalue_2 (Variables|Default|GetArrow3) "RightHand" "SnapToTarget" "SnapToTarget" "KeepWorld" true)
                              (Components|Timeline|SetPlaybackPosition (Variables|Default|GetTimeline_0) 0.25 false true)
                              (bind _newtrack_0_2 (Timeline|Timeline_0 Play)
                                (:Update
                                  (Transformation|SetRelativeRotation (Variables|Default|GetArrow) (Math|Rotator|Lerp(Rotator) "-180.000000,0.000000, 0" "0, 0, 0" _newtrack_0_2) false false))
                                (:NewTrack_1
                                  (Variables|Default|SetSwingForward/Back true))
                                (:NewTrack_2
                                  (Variables|Default|SetSwingForward/Back false))))))
                        (:then_1
                          (Utilities|FlowControl|RetriggerableDelay 0.96)
                          (Components|Animation|PlayAnimation (Variables|Default|Getgrabbable_metal_lum_for_hanging_anim1) "/Game/Blueprints/HangingPlatform/grabbable_metal_lum_for_hanging_anim1_Anim_OPENSPACE_MODEL_ARMATURE_OBJECT_OBJECT_Animation_3.grabbable_metal_lum_for_hanging_anim1_Anim_OPENSPACE_MODEL_ARMATURE_OBJECT_OBJECT_Animation_3" true)))
                      (else
                        (goto _label_3)))))
                (else
                  (CallFunction|ResetDoOnce)
                  (if (Variables|Default|GetRequiresCanPowerup)
                    (Variables|Default|SetTags (Utilities|Array|MakeArray "Target" "B"))
                    (else
                      (Variables|Default|SetTags (Utilities|Array|MakeArray "Target"))))))
              (else
                (goto _label_2))))))
      (else
        (goto _label)))))

(event Custom|Rotate
  (params (Right/Left :type Float%20%28double-precision%29))
  (if (not true)
    (Components|Timeline|SetPlayRate (Variables|Default|GetTimeline_1) (* Right/Left -1.0))
    (bind _newtrack_0 (Timeline|Timeline_1 Play)
      (:Update
        (Transformation|SetRelativeRotation (Variables|Default|GetArrow2) (Math|Rotator|Lerp(Rotator) "0, 0, 0" "0,360.000000, 0" _newtrack_0) false false)))))

(event Custom|StopHanging
  (bind _returnvalue (Game|GetPlayerCharacter 0))
  (bind _returnvalue_2 (Game|GetPlayerCharacter 0))
  (bind _asbp_rayman_pawn (Utilities|Casting|CastToBP_RaymanPawn _returnvalue))
  (bind _charactermovement (Variables|/Script/Engine.Character|GetCharacterMovement _returnvalue_2))
  (if (Variables|Default|GetRequiresCanPowerup)
    ;[1 1 1] Hide Cable
    (Variables|Default|SetTags (Utilities|Array|MakeArray "Target" "B"))
    (else
      (Variables|Default|SetTags (Utilities|Array|MakeArray "Target"))))
  (Rendering|SetVisibility (Variables|Default|GetCable) false false)
  (Utilities|FlowControl|Sequence
    (:then_0
      (bind _newtrack_0 (Timeline|Timeline_0 Stop)
        (:Update
          (Transformation|SetRelativeRotation (Variables|Default|GetArrow) (Math|Rotator|Lerp(Rotator) "-180.000000,0.000000, 0" "0, 0, 0" _newtrack_0) false false))
        (:NewTrack_1
          (Variables|Default|SetSwingForward/Back true))
        (:NewTrack_2
          (Variables|Default|SetSwingForward/Back false))))
    (:then_1
      (Utilities|FlowControl|DoOnce false) ; enters at Reset
    )
    (:then_2
      (CallFunction|ResetDoOnce))
    (:then_3
      (CallFunction|StopTimeLine))))

(event Custom|ResetDoOnce
  (bind _returnvalue (Game|GetPlayerCharacter 0))
  (bind _returnvalue_2 (Game|GetPlayerCharacter 0))
  (bind _asbp_rayman_pawn (Utilities|Casting|CastToBP_RaymanPawn _returnvalue))
  (bind _charactermovement (Variables|/Script/Engine.Character|GetCharacterMovement _returnvalue_2))
  (Utilities|FlowControl|DoOnce false) ; enters at Reset
)

(event Custom|StopTimeLine
  (bind _newtrack_0 (Timeline|Timeline_1 Stop)
    (:Update
      (Transformation|SetRelativeRotation (Variables|Default|GetArrow2) (Math|Rotator|Lerp(Rotator) "0, 0, 0" "0,360.000000, 0" _newtrack_0) false false))))

(fn ConstructionScript
  (if (Variables|Default|GetRequiresCanPowerup)
    (Rendering|SetVisibility (Variables|Default|Getgrabbable_metal_lum_for_hanging_anim1) true true)
    (Variables|Default|SetTags (Utilities|Array|MakeArray "Target" "B"))
    (Rendering|SetVisibility (Variables|Default|GetMaterialBillboard) false false)
    (Rendering|Material|SetMaterial (Variables|Default|GetCable) 0 "/Game/Textures/tex1_64x64_m_eddbc055bb575d2c_14_Mat.tex1_64x64_m_eddbc055bb575d2c_14_Mat")
    (else
      (Rendering|SetVisibility (Variables|Default|Getgrabbable_metal_lum_for_hanging_anim1) false true)
      (Variables|Default|SetTags (Utilities|Array|MakeArray "Target"))
      (Rendering|SetVisibility (Variables|Default|GetMaterialBillboard) true false)
      (Rendering|Material|SetMaterial (Variables|Default|GetCable) 0 "/Game/Textures/tex1_64x64_m_eddbc055bb575d2c_14_Mat_2.tex1_64x64_m_eddbc055bb575d2c_14_Mat_2"))))