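; Menu disc actor for the 3D main menu, with per-instance flags that hide its home disc, character disc or widget parts on BeginPlay.
; Its Menu3DWidget raises transitions by index into LinkedMenus, handing collision to the target actor and blending the camera to it.
; A portal timeline animates VFX ring material parameters and the hologram's erode.
; New game, settings and load handlers are empty, and the data-table tunnel sequence logic is disconnected.
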(event Custom|Active%20Home%20Portal
  (bind _vfx (Variables|Default|GetVFX))
  ;[1 1 1] Activate Portal
  (bind _newtrack_0 (Timeline|Timeline Play)
    (:Update
      ;;[0.4914 1 0.5337] Big Circle A
      (Utilities|LerpScalarMaterialParameterValues _vfx "Radius" 0.3 0.5 (Math|Float|Lerp 1.0 0.0 _newtrack_0))
      (Utilities|LerpScalarMaterialParameterValues _vfx "X Tile Speed" -0.02 -0.3 (Math|Float|Lerp 1.0 0.0 _newtrack_0))
      (Utilities|LerpScalarMaterialParameterValues _vfx "X Tile Speed (2)" 0.02 0.3 (Math|Float|Lerp 1.0 0.0 _newtrack_0))
      ;;[0.4914 1 0.5337] Big Circle B
      (Utilities|LerpScalarMaterialParameterValues (Variables|Default|GetVFX1%20) "Radius" 0.5 0.0 (Math|Float|Lerp 1.0 0.0 _newtrack_0))
      ;;[0.4914 1 0.5337] Big Circle C
      (Utilities|LerpScalarMaterialParameterValues (Variables|Default|GetVFX2%20) "Radius" 1.0 0.0 (Math|Float|Lerp 1.0 0.0 _newtrack_0))
      ;;[0.4914 1 0.5337] Hologram
      (bind _returnvalue (Rendering|Material|CreateDynamicMaterialInstance (Variables|Default|GetM2_HomeDisc_Object_1) 0 "/Game/Levels/Menu/HomeDisc/Material/M_Hologram.M_Hologram" "None" :!class /Script/Engine.PrimitiveComponent))
      (Rendering|Material|SetScalarParameterValue _returnvalue "Erode" _newtrack_0 :!class /Script/Engine.MaterialInstanceDynamic))))

(event Custom|TransitionTo
  (params (Transition%20Target :type BP%20Menu%20Disc%20Object%20Reference))
  ;[1 1 1] TransitionTo (Target)
  (Collision|SetActorEnableCollision false)
  (Collision|SetActorEnableCollision Transition%20Target true)
  (Game|Player|SetViewTargetwithBlend (Game|GetPlayerController 0) Transition%20Target 1.0 "VTBlend_Cubic" 0.0 true))

(event Custom|HideWidget
  ;[1 1 1] Hide Elements Chain
  ;;[1 1 1] Hide Widget
  (if (Variables|Default|GetHIDE_Widget)
    (Development|SetHiddeninGame (Variables|Default|GetWidget) true false)))

(event Custom|Hide_Elements
  ;[1 1 1] Hide Elements Chain
  (CallFunction|HideHomeDisc)
  (CallFunction|HideCharDisc)
  (CallFunction|HideWidget))

(event Custom|On%20Transition%20Between%20Menus
  (params (MenuIndex :type Integer))
  ;[1 1 1] Begin Play
  (if (Utilities|Array|IsValidIndex (Variables|Default|GetLinkedMenus) MenuIndex)
    (CallFunction|Transitionto (Utilities|Array|Get(acopy) (Variables|Default|GetLinkedMenus) MenuIndex))))

(event Custom|On%20Clicked%20%28ButtonNEWGAME%29
  ;[0.224 0.3031 1] Click New Game
)

(event Custom|HideHomeDisc
  ;[1 1 1] Hide Elements Chain
  ;;[1 1 1] HideHomeDisc
  (if (Variables|Default|GetHIDE_HomeDisc)
    (for _array_element (Utilities|Array|MakeArray (Variables|Default|GetM2_HomeDisc_Inner_Laser) (Variables|Default|GetM2_HomeDisc_Display_Border_W) (Variables|Default|GetM2_HomeDisc_Border_L) (Variables|Default|GetM2_HomeDisc_Object_1) (Variables|Default|GetFlashlight3) (Variables|Default|GetVFX2%20) (Variables|Default|GetVFX) (Variables|Default|GetVFX1%20) (Variables|Default|GetBackgroundDisc))
      (Development|SetHiddeninGame _array_element true false))))

(event Custom|Click%20Quit%20Game
  ;[0.224 0.3031 1] Quit Game
  (if (Variables|HOME|GetisPlaying_SEQ_HOME)
    (Variables|HOME|SetisPlaying_SEQ_HOME false)
    (Game|QuitGame 0 "Quit" false)))

(event Custom|Click%20Settings
  ;[0.224 0.3031 1] Click Settings
)

(event Custom|Click%20Load%20Game
  ;[0.224 0.3031 1] Load Game
)

(event Custom|HideCharDisc
  ;[1 1 1] Hide Elements Chain
  ;;[1 1 1] Hide Char Disc
  (if (Variables|Default|GetHIDE_CharDisc)
    (Development|SetHiddeninGame (Variables|Default|GetM2_CharDisc) true false)))

(event EventBeginPlay
  ;[1 1 1] Begin Play
  (CallFunction|HideElements)
  (bind _asmenu_3dwidget (Utilities|Casting|CastToMenu3DWidget (UserInterface|GetUserWidgetObject (Variables|Default|GetWidget))))
  (EventDispatchers|AssignTransitiontoLinkedMenu _asmenu_3dwidget (delegate Custom|On%20Transition%20Between%20Menus))
  (Collision|SetActorEnableCollision false))

(fn ConstructionScript)

(fn PlaySequence
  (params (Level%20Sequence :type Level%20Sequence%20Object%20Reference) (Settings%20Loop :type Movie%20Scene%20Sequence%20Loop%20Count%20Structure))
  (bind _outactor (Sequencer|Player|CreateLevelSequencePlayer Level%20Sequence (Utilities|Struct|MakeMovieSceneSequencePlaybackSettings false Settings%20Loop 1.0 0.0 false false false false false false false false)))
  (Sequencer|Player|Play (Variables|/Script/LevelSequence.LevelSequenceActor|GetSequencePlayer _outactor) :!class /Script/MovieScene.MovieSceneSequencePlayer)
  (return (Media|MediaPlayer|GetDuration (Variables|/Script/LevelSequence.LevelSequenceActor|GetSequencePlayer _outactor)) (Variables|/Script/LevelSequence.LevelSequenceActor|GetSequencePlayer _outactor)))