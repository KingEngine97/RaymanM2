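; BP_SplineRace is a spline race actor that registers itself with the player's BP_Rayman while the player is on that section.
; Beginning an overlap on the Start trigger stores that trigger's forward vector and sets Rayman's BPSplineRace reference to this actor.
; Ending an overlap on the End trigger clears that reference; both handlers use player pawn 0 without checking which actor overlapped.
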(event OnComponentBeginOverlap(Start)
  (params (OverlappedComponent :type Primitive%20Component%20Object%20Reference) (OtherActor :type Actor%20Object%20Reference) (OtherComp :type Primitive%20Component%20Object%20Reference) (OtherBodyIndex :type Integer) (bFromSweep :type Boolean) (SweepResult :type Hit%20Result%20Structure%20%28by%20ref%29))
  ;[0.4914 1 0.5337] Used
  ;;[0.4914 1 0.5337] Trigger START // Set Spline
  (Variables|Default|SetSplineStartForwardVector (Math|Vector|GetForwardVector OverlappedComponent))
  (bind _asbp_rayman (Utilities|Casting|CastToBP_Rayman (Game|Player|GetPlayerPawn 0)))
  (Variables|/Game/Characters/Rayman/BP_Rayman.BP_Rayman_C|SetBP%20SplineRace _asbp_rayman self))

(event OnComponentEndOverlap(End)
  (params (OverlappedComponent :type Primitive%20Component%20Object%20Reference) (OtherActor :type Actor%20Object%20Reference) (OtherComp :type Primitive%20Component%20Object%20Reference) (OtherBodyIndex :type Integer))
  ;[0.4914 1 0.5337] Used
  ;;[0.4914 1 0.5337] Trigger END // Un-Set Spline
  (bind _asbp_rayman (Utilities|Casting|CastToBP_Rayman (Game|Player|GetPlayerPawn 0)))
  (Variables|/Game/Characters/Rayman/BP_Rayman.BP_Rayman_C|SetBP%20SplineRace _asbp_rayman 0))

(event EventBeginPlay)

(fn ConstructionScript)