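; Blueprint function library with a single ToggleDebugInfo function that switches debug display on and off for the first player.
; It lazily creates a DebugInfo_W widget stored on InGame_PC, then adds it to or removes it from the viewport and sets the controller's DebugInfo flag to match.
; It also flips the in-game visibility of the BP_Rayman character's capsule component, independently of the widget state.
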(fn ToggleDebugInfo
  (bind _returnvalue (Game|GetPlayerController 0))
  (bind _asin_game_pc (Utilities|Casting|CastToInGame_PC _returnvalue))
  (Utilities|IsValid (Variables|/Game/Blueprint/PlayerController/InGame_PC.InGame_PC_C|GetDebugInfo_W (.AsIn%20Game%20PC (Utilities|Casting|CastToInGame_PC (Game|GetPlayerController 0))))
    (:Is%20Valid
      _)
    (:Is%20Not%20Valid
      (bind _returnvalue_2 (UserInterface|CreateWidget "/Game/Blueprint/Function/DebugInfo_W.DebugInfo_W_C"))
      (Variables|/Game/Blueprint/PlayerController/InGame_PC.InGame_PC_C|SetDebugInfo_W (.AsIn%20Game%20PC (Utilities|Casting|CastToInGame_PC (Game|GetPlayerController 0))) _returnvalue_2)))
  (if (UserInterface|Viewport|IsinViewport (Variables|/Game/Blueprint/PlayerController/InGame_PC.InGame_PC_C|GetDebugInfo_W _asin_game_pc))
    (Widget|RemovefromParent (Variables|/Game/Blueprint/PlayerController/InGame_PC.InGame_PC_C|GetDebugInfo_W _asin_game_pc))
    (Variables|/Game/Blueprint/PlayerController/InGame_PC.InGame_PC_C|SetDebugInfo _asin_game_pc false)
    (else
      (UserInterface|Viewport|AddtoViewport (Variables|/Game/Blueprint/PlayerController/InGame_PC.InGame_PC_C|GetDebugInfo_W _asin_game_pc) 12)
      (Variables|/Game/Blueprint/PlayerController/InGame_PC.InGame_PC_C|SetDebugInfo _asin_game_pc true)))
  (bind _asbp_rayman_pawn (Utilities|Casting|CastToBP_Rayman (Game|GetPlayerCharacter 0)))
  (Utilities|IsValid _asbp_rayman_pawn
    (:Is%20Valid
      (Development|SetHiddeninGame (Variables|/Script/Engine.Character|GetCapsuleComponent _asbp_rayman_pawn) (not (Variables|/Script/Engine.SceneComponent|GetbHiddenInGame (Variables|/Script/Engine.Character|GetCapsuleComponent _asbp_rayman_pawn))) false))))