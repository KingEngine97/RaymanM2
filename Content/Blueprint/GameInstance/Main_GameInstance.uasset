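; Game instance that persists story progress and player settings through SaveGame_BP objects in separate progress and config slots.
; SaveGame records the trigger, load flag and optionally current level and BGM, then plays the battle HUD's save animation.
; SaveGameSettings and LoadGameSettings copy graphics, audio and voice-language values to and from the config slot.
; Init loads settings, but its LoadGame call is empty; story-loading logic sits in an uncalled CustomEvent.
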(event Custom|SaveGame
  (params (SaveGameTriggerID :type Integer) (StoryMode_EnableLoadGame :type Boolean) (SaveCurrentLevel :type Boolean) (BGMToLoad :type Sound%20Base%20Object%20Reference))
  (Variables|Default|SetStoryMode_SaveGameOnNextLevel false)
  (Variables|Default|SetStoryMode_CurrentSaveGameTrigger SaveGameTriggerID)
  (Variables|Default|SetStoryMode_LoadGameEnabled StoryMode_EnableLoadGame)
  (bind _returnvalue (SaveGame|DoesSaveGameExist "RAYMANLE00"))
  (if _returnvalue
    (bind _returnvalue_2 (SaveGame|LoadGamefromSlot "RAYMANLE00"))
    (bind _assave_game_bp (Utilities|Casting|CastToSaveGame_BP _returnvalue_2))
    (Variables|Default|SetSaveGameBP _assave_game_bp)
    (else
      (bind _returnvalue_3 (SaveGame|CreateSaveGameObject "/Game/Blueprint/GameInstance/SaveGame_BP.SaveGame_BP_C"))
      (Variables|Default|SetSaveGameBP _returnvalue_3)))
  (Variables|/Game/Blueprint/GameInstance/SaveGame_BP.SaveGame_BP_C|SetStoryMode_CurrentSaveGameTrigger (Variables|Default|GetSaveGameBP) (Variables|Default|GetStoryMode_CurrentSaveGameTrigger))
  (if SaveCurrentLevel
    (bind _returnvalue_4 (Game|GetCurrentLevelName true))
    (Variables|/Game/Blueprint/GameInstance/SaveGame_BP.SaveGame_BP_C|SetStoryMode_CurrentLevel (Variables|Default|GetSaveGameBP) _returnvalue_4)
    (Variables|/Game/Blueprint/GameInstance/SaveGame_BP.SaveGame_BP_C|SetCurrentBGM (Variables|Default|GetSaveGameBP) BGMToLoad))
  (Variables|/Game/Blueprint/GameInstance/SaveGame_BP.SaveGame_BP_C|SetStoryMode_LoadGameEnabled (Variables|Default|GetSaveGameBP) (Variables|Default|GetStoryMode_LoadGameEnabled))
  (SaveGame|SaveGametoSlot (Variables|Default|GetSaveGameBP) "RAYMANLE00")
  (bind _foundwidgets (Widget|GetAllWidgetsOfClass "/Game/Level/Menu/U-Interface/InGame_Battle_W.InGame_Battle_W_C" true))
  (Utilities|IsValid (Utilities|Array|Get(acopy) _foundwidgets)
    (:Is%20Valid
      (UserInterface|Animation|PlayAnimation (Utilities|Array|Get(acopy) _foundwidgets) (Variables|/Game/Level/Menu/U-Interface/InGame_Battle_W.InGame_Battle_W_C|GetSaveAnimation (Utilities|Array|Get(acopy) _foundwidgets)) 0.0 1 "Forward" 1.0 false))))

(event Custom|SaveGameSettings
  (bind _returnvalue (SaveGame|DoesSaveGameExist "RAYMANLE_Config"))
  (if _returnvalue
    (bind _returnvalue_2 (SaveGame|LoadGamefromSlot "RAYMANLE_Config"))
    (bind _assave_game_bp (Utilities|Casting|CastToSaveGame_BP _returnvalue_2))
    (Variables|Default|SetSaveGameBP _assave_game_bp)
    (else
      (bind _returnvalue_3 (SaveGame|CreateSaveGameObject "/Game/Blueprint/GameInstance/SaveGame_BP.SaveGame_BP_C"))
      (Variables|Default|SetSaveGameBP _returnvalue_3)))
  (Variables|/Game/Blueprint/GameInstance/SaveGame_BP.SaveGame_BP_C|SetGlobalIlluminationQuality (Variables|Default|GetSaveGameBP) (Variables|Default|GetGlobalIlluminationQuality))
  (Variables|/Game/Blueprint/GameInstance/SaveGame_BP.SaveGame_BP_C|SetShadowQuality (Variables|Default|GetSaveGameBP) (Variables|Default|GetShadowQuality))
  (Variables|/Game/Blueprint/GameInstance/SaveGame_BP.SaveGame_BP_C|SetRayTracingQuality (Variables|Default|GetSaveGameBP) (Variables|Default|GetRayTracingQuality))
  (Variables|/Game/Blueprint/GameInstance/SaveGame_BP.SaveGame_BP_C|SetShadingQuality (Variables|Default|GetSaveGameBP) (Variables|Default|GetShadingQuality))
  (Variables|/Game/Blueprint/GameInstance/SaveGame_BP.SaveGame_BP_C|SetTextureQuality (Variables|Default|GetSaveGameBP) (Variables|Default|GetTextureQuality))
  (Variables|/Game/Blueprint/GameInstance/SaveGame_BP.SaveGame_BP_C|SetResolution (Variables|Default|GetSaveGameBP) (Variables|Default|GetResolution))
  (Variables|/Game/Blueprint/GameInstance/SaveGame_BP.SaveGame_BP_C|SetCurrentVoiceLanguage (Variables|Default|GetSaveGameBP) (Variables|Default|GetCurrentVoiceLanguage))
  (Variables|/Game/Blueprint/GameInstance/SaveGame_BP.SaveGame_BP_C|SetSND_MasterVolume (Variables|Default|GetSaveGameBP) (Variables|Default|GetSND_MasterVolume))
  (Variables|/Game/Blueprint/GameInstance/SaveGame_BP.SaveGame_BP_C|SetSND_MusicVolume (Variables|Default|GetSaveGameBP) (Variables|Default|GetSND_MusicVolume))
  (Variables|/Game/Blueprint/GameInstance/SaveGame_BP.SaveGame_BP_C|SetSND_SFXVolume (Variables|Default|GetSaveGameBP) (Variables|Default|GetSND_SFXVolume))
  (Variables|/Game/Blueprint/GameInstance/SaveGame_BP.SaveGame_BP_C|SetSND_DialogueVolume (Variables|Default|GetSaveGameBP) (Variables|Default|GetSND_DialogueVolume))
  (Variables|/Game/Blueprint/GameInstance/SaveGame_BP.SaveGame_BP_C|SetFullscreen (Variables|Default|GetSaveGameBP) (Variables|Default|GetFullscreen))
  (Variables|/Game/Blueprint/GameInstance/SaveGame_BP.SaveGame_BP_C|SetVsync (Variables|Default|GetSaveGameBP) (Variables|Default|GetVsync))
  (Variables|/Game/Blueprint/GameInstance/SaveGame_BP.SaveGame_BP_C|SetMaxFPS (Variables|Default|GetSaveGameBP) (Variables|Default|GetMaxFPS))
  (Variables|/Game/Blueprint/GameInstance/SaveGame_BP.SaveGame_BP_C|SetAAQuality (Variables|Default|GetSaveGameBP) (Variables|Default|GetAAQuality))
  (Variables|/Game/Blueprint/GameInstance/SaveGame_BP.SaveGame_BP_C|SetAAMethod (Variables|Default|GetSaveGameBP) (Variables|Default|GetAAMethod))
  (SaveGame|SaveGametoSlot (Variables|Default|GetSaveGameBP) "RAYMANLE_Config"))

(event Custom|CustomEvent
  (bind _returnvalue (SaveGame|DoesSaveGameExist "RAYMANLE00"))
  (if _returnvalue
    (bind _returnvalue_2 (SaveGame|LoadGamefromSlot "RAYMANLE00"))
    (bind _assave_game_bp (Utilities|Casting|CastToSaveGame_BP _returnvalue_2))
    (bind _output_get (Variables|Default|SetSaveGameBP _assave_game_bp))
    (Variables|Default|SetStoryMode_CurrentSaveGameTrigger (Variables|/Game/Blueprint/GameInstance/SaveGame_BP.SaveGame_BP_C|GetStoryMode_CurrentSaveGameTrigger _output_get))
    (Variables|Default|SetStoryMode_CurrentLevel (Variables|/Game/Blueprint/GameInstance/SaveGame_BP.SaveGame_BP_C|GetStoryMode_CurrentLevel _output_get))
    (Variables|Default|SetStoryMode_LoadGameEnabled (Variables|/Game/Blueprint/GameInstance/SaveGame_BP.SaveGame_BP_C|GetStoryMode_LoadGameEnabled _output_get))
    (else
      (bind _returnvalue_3 (SaveGame|CreateSaveGameObject "/Game/Blueprint/GameInstance/SaveGame_BP.SaveGame_BP_C"))
      (Variables|Default|SetSaveGameBP _returnvalue_3))))

(event Custom|LoadGameSettings
  (bind _returnvalue (SaveGame|DoesSaveGameExist "RAYMANLE_Config"))
  (if _returnvalue
    (bind _returnvalue_2 (SaveGame|LoadGamefromSlot "RAYMANLE_Config"))
    (bind _assave_game_bp (Utilities|Casting|CastToSaveGame_BP _returnvalue_2))
    (bind _output_get (Variables|Default|SetSaveGameBP _assave_game_bp))
    (Variables|Default|SetGlobalIlluminationQuality (Variables|/Game/Blueprint/GameInstance/SaveGame_BP.SaveGame_BP_C|GetGlobalIlluminationQuality _output_get))
    (Variables|Default|SetShadowQuality (Variables|/Game/Blueprint/GameInstance/SaveGame_BP.SaveGame_BP_C|GetShadowQuality _output_get))
    (Variables|Default|SetRayTracingQuality (Variables|/Game/Blueprint/GameInstance/SaveGame_BP.SaveGame_BP_C|GetRayTracingQuality _output_get))
    (Variables|Default|SetShadingQuality (Variables|/Game/Blueprint/GameInstance/SaveGame_BP.SaveGame_BP_C|GetShadingQuality _output_get))
    (Variables|Default|SetTextureQuality (Variables|/Game/Blueprint/GameInstance/SaveGame_BP.SaveGame_BP_C|GetTextureQuality _output_get))
    (Variables|Default|SetResolution (Variables|/Game/Blueprint/GameInstance/SaveGame_BP.SaveGame_BP_C|GetResolution _output_get))
    (Variables|Default|SetCurrentVoiceLanguage (Variables|/Game/Blueprint/GameInstance/SaveGame_BP.SaveGame_BP_C|GetCurrentVoiceLanguage _output_get))
    (Variables|Default|SetSND_MasterVolume (Variables|/Game/Blueprint/GameInstance/SaveGame_BP.SaveGame_BP_C|GetSND_MasterVolume _output_get))
    (Variables|Default|SetSND_MusicVolume (Variables|/Game/Blueprint/GameInstance/SaveGame_BP.SaveGame_BP_C|GetSND_MusicVolume _output_get))
    (Variables|Default|SetSND_SFXVolume (Variables|/Game/Blueprint/GameInstance/SaveGame_BP.SaveGame_BP_C|GetSND_SFXVolume _output_get))
    (Variables|Default|SetSND_DialogueVolume (Variables|/Game/Blueprint/GameInstance/SaveGame_BP.SaveGame_BP_C|GetSND_DialogueVolume _output_get))
    (Variables|Default|SetFullscreen (Variables|/Game/Blueprint/GameInstance/SaveGame_BP.SaveGame_BP_C|GetFullscreen _output_get))
    (Variables|Default|SetVsync (Variables|/Game/Blueprint/GameInstance/SaveGame_BP.SaveGame_BP_C|GetVsync _output_get))
    (Variables|Default|SetMaxFPS (Variables|/Game/Blueprint/GameInstance/SaveGame_BP.SaveGame_BP_C|GetMaxFPS _output_get))
    (Variables|Default|SetAAMethod (Variables|/Game/Blueprint/GameInstance/SaveGame_BP.SaveGame_BP_C|GetAAMethod _output_get))
    (Variables|Default|SetAAQuality (Variables|/Game/Blueprint/GameInstance/SaveGame_BP.SaveGame_BP_C|GetAAQuality _output_get))
    (else
      (bind _returnvalue_3 (SaveGame|CreateSaveGameObject "/Game/Blueprint/GameInstance/SaveGame_BP.SaveGame_BP_C"))
      (Variables|Default|SetSaveGameBP _returnvalue_3))))

(event EventInit
  (CallFunction|LoadGame)
  (CallFunction|LoadGameSettings))

(fn LoadGame)