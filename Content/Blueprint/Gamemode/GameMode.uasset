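; Game mode for a Rayman game that applies graphics settings and plays cutscenes.
; UpdateGraphics turns values stored in Main_GameInstance into scalability, resolution, VSync, frame-cap and anti-aliasing console commands.
; PlayCutscene disables player input, optionally hides BP_RaymanPawn, waits out the Level Sequence, then restores the pawn with an optional teleport.
; BeginPlay is empty; disconnected logic remains for save-trigger loading, level streaming and character spawning.
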(event Custom|UpdateGraphics
  (bind _returnvalue (Game|GetGameInstance))
  (bind _asmain_game_instance (Utilities|Casting|CastToMain_GameInstance _returnvalue))
  (Development|ExecuteConsoleCommand (Utilities|String|Append "sg.ShadowQuality " (Utilities|String|ToString(Integer) (Variables|/Game/Blueprint/GameInstance/Main_GameInstance.Main_GameInstance_C|GetShadowQuality (.AsMain%20Game%20Instance (Utilities|Casting|CastToMain_GameInstance (Game|GetGameInstance)))))) 0)
  (Development|ExecuteConsoleCommand (Utilities|String|Append "sg.GlobalIlluminationQuality " (Utilities|String|ToString(Integer) (Variables|/Game/Blueprint/GameInstance/Main_GameInstance.Main_GameInstance_C|GetGlobalIlluminationQuality (.AsMain%20Game%20Instance (Utilities|Casting|CastToMain_GameInstance (Game|GetGameInstance)))))) 0)
  (Development|ExecuteConsoleCommand (Utilities|String|Append "sg.ShadingQuality " (Utilities|String|ToString(Integer) (Variables|/Game/Blueprint/GameInstance/Main_GameInstance.Main_GameInstance_C|GetShadingQuality (.AsMain%20Game%20Instance (Utilities|Casting|CastToMain_GameInstance (Game|GetGameInstance)))))) 0)
  (Development|ExecuteConsoleCommand (Utilities|String|Append "sg.EffectsQuality " (Utilities|String|ToString(Integer) (Variables|/Game/Blueprint/GameInstance/Main_GameInstance.Main_GameInstance_C|GetShadingQuality (.AsMain%20Game%20Instance (Utilities|Casting|CastToMain_GameInstance (Game|GetGameInstance)))))) 0)
  (Development|ExecuteConsoleCommand (Utilities|String|Append "sg.PostProcessQuality " (Utilities|String|ToString(Integer) (Variables|/Game/Blueprint/GameInstance/Main_GameInstance.Main_GameInstance_C|GetShadowQuality (.AsMain%20Game%20Instance (Utilities|Casting|CastToMain_GameInstance (Game|GetGameInstance)))))) 0)
  (Development|ExecuteConsoleCommand (Utilities|String|Append "sg.TextureQuality " (Utilities|String|ToString(Integer) (Variables|/Game/Blueprint/GameInstance/Main_GameInstance.Main_GameInstance_C|GetTextureQuality (.AsMain%20Game%20Instance (Utilities|Casting|CastToMain_GameInstance (Game|GetGameInstance)))))) 0)
  (Development|ExecuteConsoleCommand (Utilities|String|Append "r.SetRes " (Utilities|Select :Index (Variables|/Game/Blueprint/GameInstance/Main_GameInstance.Main_GameInstance_C|GetResolution _asmain_game_instance) :Option%200 "960x540" :Option%201 "1024x640" :Option%202 "1024x576" :Option%203 "1152x720" :Option%204 "1280x720" :Option%205 "1280x800" :Option%206 "1600x900" :Option%207 "1920x1080") (Utilities|String|SelectString "f" "w" (Math|Conversions|ToBoolean(Integer) (Variables|/Game/Blueprint/GameInstance/Main_GameInstance.Main_GameInstance_C|GetResolution _asmain_game_instance)))) 0)
  (Development|ExecuteConsoleCommand (Utilities|String|Append "r.VSync " (Utilities|String|ToString(Integer) (Variables|/Game/Blueprint/GameInstance/Main_GameInstance.Main_GameInstance_C|GetVsync (.AsMain%20Game%20Instance (Utilities|Casting|CastToMain_GameInstance (Game|GetGameInstance)))))) 0)
  (Development|ExecuteConsoleCommand (Utilities|String|Append "t.MaxFPS " (Utilities|String|ToString(Float) (Utilities|Select :Index (Variables|/Game/Blueprint/GameInstance/Main_GameInstance.Main_GameInstance_C|GetMaxFPS (.AsMain%20Game%20Instance (Utilities|Casting|CastToMain_GameInstance (Game|GetGameInstance)))) :Option%200 4e+02 :Option%201 3e+01 :Option%202 4e+01 :Option%203 6e+01 :Option%204 1.2e+02 :Option%205 144.0))) 0)
  (Development|ExecuteConsoleCommand (Utilities|String|Append "r.AntiAliasingMethod " (Utilities|String|SelectString "2" "1" (Math|Conversions|ToBoolean(Integer) (Variables|/Game/Blueprint/GameInstance/Main_GameInstance.Main_GameInstance_C|GetAAMethod (.AsMain%20Game%20Instance (Utilities|Casting|CastToMain_GameInstance (Game|GetGameInstance))))))) 0)
  (Development|ExecuteConsoleCommand (Utilities|String|Append "sg.AntiAliasingQuality " (Utilities|Select :Index (Variables|/Game/Blueprint/GameInstance/Main_GameInstance.Main_GameInstance_C|GetAAQuality (.AsMain%20Game%20Instance (Utilities|Casting|CastToMain_GameInstance (Game|GetGameInstance)))) :Option%200 "0" :Option%201 "2" :Option%202 "3" :Option%203 "4")) 0))

(event Custom|PlayCutscene
  (params (Cutscene :type Level%20Sequence%20Object%20Reference) (TeleportPlayerAfterCutscene :type Boolean) (TeleportPlayerToLocation :type Transform) (HidePlayer :type Boolean))
  (bind (_location _rotation) (Math|Transform|BreakTransform TeleportPlayerToLocation))
  (bind _asbp_rayman_pawn (Utilities|Casting|CastToBP_RaymanPawn (Game|GetPlayerCharacter 0)))
  (Input|DisableInput _asbp_rayman_pawn (Game|GetPlayerController 0))
  (Components|Movement|StopMovementImmediately (Variables|/Script/Engine.Character|GetCharacterMovement _asbp_rayman_pawn))
  (if HidePlayer
    (Rendering|SetActorHiddenInGame _asbp_rayman_pawn true))
  (bind _outactor (Sequencer|Player|CreateLevelSequencePlayer Cutscene))
  (Sequencer|Player|Play (Variables|/Script/LevelSequence.LevelSequenceActor|GetSequencePlayer _outactor) :!class /Script/MovieScene.MovieSceneSequencePlayer)
  (Utilities|FlowControl|Delay (Class|TimeManagementBlueprintLibrary|ToSeconds(QualifiedFrameTime) (Media|MediaPlayer|GetDuration (Variables|/Script/LevelSequence.LevelSequenceActor|GetSequencePlayer _outactor))))
  (if TeleportPlayerAfterCutscene
    (bind _asbp_rayman_pawn_2 (Utilities|Casting|CastToBP_RaymanPawn (Game|GetPlayerCharacter 0)))
    (Transformation|SetActorLocationAndRotation _asbp_rayman_pawn_2 _location _rotation false true)
    (Rendering|SetActorHiddenInGame _asbp_rayman_pawn_2 false)
    (Input|EnableInput _asbp_rayman_pawn_2 (Game|GetPlayerController 0))
    (else
      (bind _asbp_rayman_pawn_3 (Utilities|Casting|CastToBP_RaymanPawn (Game|GetPlayerCharacter 0)))
      (Rendering|SetActorHiddenInGame _asbp_rayman_pawn_3 false)
      (Input|EnableInput _asbp_rayman_pawn_3 (Game|GetPlayerController 0)))))

(event EventBeginPlay
  ;[1 0.3177 0.3177] Comment
  ;;[1 1 1] Comment
)

(fn ConstructionScript)