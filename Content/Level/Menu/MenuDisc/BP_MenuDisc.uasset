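; Menu disc Blueprint that drives the menu's move from Home to Online through Level Sequences, starting the Home sequence on BeginPlay.
; Clicking the ONLINE button runs a timeline that erodes several holograms, then stops Home and plays the HomeToOnline transition.
; A gate switches to the Online sequence on a mouse press or after the transition's duration, and mouse release closes it.
; Hovering ONLINE sets its material highlight colors, reverting to black afterward.
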(event OnClicked(ButtonONLINE)
  (params (TouchedComponent :type Primitive%20Component%20Object%20Reference) (ButtonPressed :type Key%20Structure :default "None"))
  (bind _add_erode (Timeline|Timeline Play)
    (:Update
      ;[1 1 1] Click Online
      (Rendering|Material|SetScalarParameterValueonMaterials (Variables|Default|GetHologram1) "add erode" _add_erode))
    (:Finished
      (Variables|ONLINE|SetSkip%20"SEQ_Home_to_Online" true)
      (Sequencer|Player|Stop (stale EventBeginPlay _sequence_player_out) :!class /Script/MovieScene.MovieSceneSequencePlayer)
      (bind (_sequence_duration _sequence_player_out) (CallFunction|PlaySequence (Variables|ONLINE|GetSEQ_Home_to_Online)))
      (if (Variables|ONLINE|GetSkip%20"SEQ_Home_to_Online")
        (Utilities|FlowControl|Sequence
          (:then_0
            (goto _label Open))
          (:then_1
            (Utilities|FlowControl|Delay (Class|TimeManagementBlueprintLibrary|ToSeconds(QualifiedFrameTime) _sequence_duration))
            (Utilities|FlowControl|Gate true :!label _label
              (:Exit
                (Sequencer|Player|Stop _sequence_player_out :!class /Script/MovieScene.MovieSceneSequencePlayer)
                ;;[1 1 1] Play "SEQ_Online"
                (CallFunction|PlaySequence (Variables|ONLINE|GetSEQ_Online) (Variables|Default|GetSettings%20Loop))
                (Variables|Default|SetIsUsingMenuOnline true)))))))))

(event OnBeginCursorOver(ButtonONLINE)
  (params (TouchedComponent :type Primitive%20Component%20Object%20Reference))
  (bind _buttononline (Utilities|HighlightButton (Variables|Default|GetButtonONLINE))))

(event OnEndCursorOver(ButtonONLINE)
  (params (TouchedComponent :type Primitive%20Component%20Object%20Reference))
  (Utilities|UnHighlightButton (stale OnBeginCursorOver(ButtonONLINE) _buttononline) (stale OnBeginCursorOver(ButtonONLINE) _buttononline)))

(event EventBeginPlay
  ;[1 1 1] Play Home Sequence
  (bind _sequence_player_out (CallFunction|PlaySequence (Variables|HOME|GetSEQ_Home) (Variables|Default|GetSettings%20Loop))))

(event Input|MouseEvents|RightMouseButton
  (params (Key :type Key%20Structure :default "None"))
  ;[1 1 1] Click Online
  (:Pressed
    (Utilities|FlowControl|Gate true :!label _label
      (:Exit
        (Sequencer|Player|Stop (stale OnClicked(ButtonONLINE) _sequence_player_out) :!class /Script/MovieScene.MovieSceneSequencePlayer)
        ;;[1 1 1] Play "SEQ_Online"
        (CallFunction|PlaySequence (Variables|ONLINE|GetSEQ_Online) (Variables|Default|GetSettings%20Loop))
        (Variables|Default|SetIsUsingMenuOnline true))))
  (:Released
    (goto _label Close)))

(event Input|MouseEvents|LeftMouseButton
  (params (Key :type Key%20Structure :default "None"))
  ;[1 1 1] Click Online
  (:Pressed
    (Utilities|FlowControl|Gate true :!label _label
      (:Exit
        (Sequencer|Player|Stop (stale OnClicked(ButtonONLINE) _sequence_player_out) :!class /Script/MovieScene.MovieSceneSequencePlayer)
        ;;[1 1 1] Play "SEQ_Online"
        (CallFunction|PlaySequence (Variables|ONLINE|GetSEQ_Online) (Variables|Default|GetSettings%20Loop))
        (Variables|Default|SetIsUsingMenuOnline true))))
  (:Released
    (goto _label Close)))

(fn ConstructionScript)

(fn PlaySequence
  (params (Level%20Sequence :type Level%20Sequence%20Object%20Reference) (Settings%20Loop :type Movie%20Scene%20Sequence%20Loop%20Count%20Structure))
  (bind _outactor (Sequencer|Player|CreateLevelSequencePlayer Level%20Sequence (Utilities|Struct|MakeMovieSceneSequencePlaybackSettings false Settings%20Loop 1.0 0.0 false false false false false false false false)))
  (Sequencer|Player|Play (Variables|/Script/LevelSequence.LevelSequenceActor|GetSequencePlayer _outactor) :!class /Script/MovieScene.MovieSceneSequencePlayer)
  (return (Media|MediaPlayer|GetDuration (Variables|/Script/LevelSequence.LevelSequenceActor|GetSequencePlayer _outactor)) (Variables|/Script/LevelSequence.LevelSequenceActor|GetSequencePlayer _outactor)))